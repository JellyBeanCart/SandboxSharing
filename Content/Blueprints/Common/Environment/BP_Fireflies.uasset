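; BP_Fireflies is an environment actor that shows a Niagara firefly effect at night while the player is inside its activation box.
; A looping timer, running while the player overlaps the box, samples NightAmbientCurve at the weather system's current time to toggle the effect.
; When active, it feeds player position and camera direction as avoidance inputs, plus an optional attractor's position and force.
; The construction script sizes the box and effect radii and sets the height.
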(event `self.ReceiveBeginPlay`
  (if (`PrimitiveComponent.IsOverlappingActor` (`self.Box`) (`/Game/Blueprints/FunctionLibrary/BP_FunctionLibrary.GetPlayerCharacter`))
    (`self.ForceCheckTime`)))

(event `ForceCheckTime`
  (bind _returnvalue (`KismetSystemLibrary.K2_SetTimerDelegate` (`|CreateDelegate` :!event `CheckTime`) 0.2 true :!label _label))
  (set `self.CheckWeatherTimer` _returnvalue))

(event `self.Box.OnComponentBeginOverlap`
  (params (OverlappedComponent :type "PrimitiveComponent Object Reference") (OtherActor :type "Actor Object Reference") (OtherComp :type "PrimitiveComponent Object Reference") (OtherBodyIndex :type Integer) (bFromSweep :type Boolean) (SweepResult :type "HitResult Structure (by ref)"))
  (cast `/Game/Blueprints/Core/BP_PlayerCharacter` OtherActor)
  (goto _label))

(event `self.Box.OnComponentEndOverlap`
  (params (OverlappedComponent :type "PrimitiveComponent Object Reference") (OtherActor :type "Actor Object Reference") (OtherComp :type "PrimitiveComponent Object Reference") (OtherBodyIndex :type Integer))
  (cast `/Game/Blueprints/Core/BP_PlayerCharacter` OtherActor)
  (`KismetSystemLibrary.K2_ClearAndInvalidateTimerHandle` (`self.CheckWeatherTimer`))
  (`ActorComponent.Deactivate` (`self.Niagara`)))

(event `CheckTime`
  (bind (_returnvalue_x _returnvalue_y) (`KismetMathLibrary.BreakVector` (`CurveVector.GetVectorValue` (`self.NightAmbientCurve`) (`/Game/Blueprints/Common/WeatherSystem/BP_WeatherSystem.CurrentTime` (`/Game/Blueprints/FunctionLibrary/BP_FunctionLibrary.GetWeatherSystem`)))))
  (if (`KismetMathLibrary.NearlyEqual_FloatFloat` _returnvalue_y 1.0)
    (`ActorComponent.Activate` (`self.Niagara`) false)
    (`NiagaraComponent.SetVariableVec3` (`self.Niagara`) "AvoidPosition" (`self.K2_GetActorLocation` (`GameplayStatics.GetPlayerCharacter` 0)))
    (`NiagaraComponent.SetVariableVec3` (`self.Niagara`) "AvoidDirection" (`KismetMathLibrary.GetForwardVector` (`PlayerCameraManager.GetCameraRotation` (`GameplayStatics.GetPlayerCameraManager` 0))))
    (`/Engine/EditorBlueprintResources/StandardMacros.IsValid` (`self.Attractor`)
      (:`Is Valid`
        (if (`/Game/Blueprints/Common/Environment/BP_OutdoorLight.Active` (`self.Attractor`))
          (`NiagaraComponent.SetVariableFloat` (`self.Niagara`) "AttractionForce" (`self.AttractionForce`))
          (`NiagaraComponent.SetVariableVec3` (`self.Niagara`) "AttractorPosition" (`self.K2_GetActorLocation` (`self.Attractor`)))
          (else
            (`NiagaraComponent.SetVariableFloat` (`self.Niagara`) "AttractionForce" 0.0)))))
    (else
      (`ActorComponent.Deactivate` (`self.Niagara`)))))

(fn `UserConstructionScript`
  (bind _activationzone (`self.ActivationZone`))
  (bind (_relativelocation_x _relativelocation_y) (`KismetMathLibrary.BreakVector` (`SceneComponent.RelativeLocation` (`self.Niagara`))))
  (`NiagaraComponent.SetVariableFloat` (`self.Niagara`) "SpawnRadius" (/ (`self.SpawnRadius`) 2.0))
  (`NiagaraComponent.SetVariableFloat` (`self.Niagara`) "KillRadius" (/ (`self.ActivationZone`) 2.0))
  (`NiagaraComponent.SetVariableFloat` (`self.Niagara`) "AttractionRadius" (/ (`self.AttractionRadius`) 2.0))
  (`BoxComponent.SetBoxExtent` (`self.Box`) (`KismetMathLibrary.MakeVector` _activationzone _activationzone 200.0) true)
  (`SceneComponent.K2_SetRelativeLocation` (`self.Niagara`) (`KismetMathLibrary.MakeVector` _relativelocation_x _relativelocation_y (`self.HeightOffset`)) false false))