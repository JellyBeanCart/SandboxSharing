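; BP_OutdoorLight is an environment Blueprint that tracks whether an outdoor light should be active based on the time of day.
; A looping timer started on BeginPlay periodically checks the weather system's current time against NightAmbientCurve.
; It sets Active to true only while the curve's X value is nearly one, and false otherwise.
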(event `self.ReceiveBeginPlay`
  (bind _returnvalue (`KismetSystemLibrary.K2_SetTimerDelegate` (`|CreateDelegate` :!event `CheckTime`) 0.2 true))
  (set `self.CheckTimeTimer` _returnvalue))

(event `CheckTime`
  (bind _returnvalue_x (`KismetMathLibrary.BreakVector` (`CurveVector.GetVectorValue` (`self.NightAmbientCurve`) (`/Game/Blueprints/Common/WeatherSystem/BP_WeatherSystem.CurrentTime` (`/Game/Blueprints/FunctionLibrary/BP_FunctionLibrary.GetWeatherSystem`)))))
  (if (`KismetMathLibrary.NearlyEqual_FloatFloat` _returnvalue_x 1.0)
    (set `self.Active` true)
    (else
      (set `self.Active` false))))

(fn `UserConstructionScript`)