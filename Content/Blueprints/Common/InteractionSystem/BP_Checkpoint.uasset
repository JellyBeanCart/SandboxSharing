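; Interactable checkpoint that saves game progress, configured by CheckpointType as Direct, AOE or Endpoint.
; Direct saves and shows the save widget on interaction; Endpoint saves and opens the target level if the player's quest component allows the next chapter.
; AOE reports to the quest component on player overlap, then saves, while the Editor flag suppresses saving and level travel.
; The construction script toggles sphere, mesh and widget per type.
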(event `self.ReceiveBeginPlay`
  (`parent.ReceiveBeginPlay`)
  (switch `/Game/Blueprints/Enumerations/ECheckpointType` (`self.CheckpointType`)
    (:`NewEnumerator1`
      (`PrimitiveComponent.SetCollisionEnabled` (`self.AOE`) "NoCollision" :!label _label))
    (:`NewEnumerator2`
      (`PrimitiveComponent.SetCollisionEnabled` (`self.AOE`) "QueryOnly"))
    (:`NewEnumerator3`
      (goto _label))))

(event `self.MainBody`
  (`parent.MainBody`)
  (switch `/Game/Blueprints/Enumerations/ECheckpointType` (`self.CheckpointType`)
    (:`NewEnumerator1`
      (if (not (`self.bEditor`))
        (message `/Game/Blueprints/Interfaces/BPI_GameInstance.SaveGameData` (`GameplayStatics.GetGameInstance`))
        (message `/Game/Blueprints/Interfaces/BPI_InteractionSystem.CreateSaveWidget` (`GameplayStatics.GetPlayerController` 0))))
    (:`NewEnumerator3`
      (if (not (`self.bEditor`))
        (if (`/Game/Blueprints/Common/QuestSystem/BP_QuestComponent.bGoNextChapter` (`self.GetComponentByClass` (`GameplayStatics.GetPlayerCharacter` 0) "/Game/Blueprints/Common/QuestSystem/BP_QuestComponent.BP_QuestComponent_C"))
          (message `/Game/Blueprints/Interfaces/BPI_GameInstance.SaveGameData` (`GameplayStatics.GetGameInstance`))
          (`GameplayStatics.OpenLevel` (`KismetStringLibrary.Conv_StringToName` (`self.Level`))))))))

(event `self.AOE.OnComponentBeginOverlap`
  (params (OverlappedComponent :type "PrimitiveComponent Object Reference") (OtherActor :type "Actor Object Reference") (OtherComp :type "PrimitiveComponent Object Reference") (OtherBodyIndex :type Integer) (bFromSweep :type Boolean) (SweepResult :type "HitResult Structure (by ref)"))
  (cast `/Game/Blueprints/Core/BP_PlayerCharacter` OtherActor)
  (`/Game/Blueprints/Common/QuestSystem/BP_QuestComponent.OnCheckpointReached` (`self.GetComponentByClass` (`GameplayStatics.GetPlayerCharacter` 0) "/Game/Blueprints/Common/QuestSystem/BP_QuestComponent.BP_QuestComponent_C") "NewEnumerator2" (`GameplayStatics.GetObjectClass` self))
  (if (not (`self.bEditor`))
    (message `/Game/Blueprints/Interfaces/BPI_GameInstance.SaveGameData` (`GameplayStatics.GetGameInstance`))
    (message `/Game/Blueprints/Interfaces/BPI_InteractionSystem.CreateSaveWidget` (`GameplayStatics.GetPlayerController` 0))))

(fn `UserConstructionScript`
  (`parent.UserConstructionScript`)
  (switch `/Game/Blueprints/Enumerations/ECheckpointType` (`self.CheckpointType`)
    (:`NewEnumerator1`
      (`SceneComponent.SetVisibility` (`self.AOE`) false false :!label _label)
      (`StaticMeshComponent.SetStaticMesh` (`self.StaticMesh`) (`self.Model`)))
    (:`NewEnumerator2`
      (`SceneComponent.SetVisibility` (`self.AOE`) true false)
      (`SphereComponent.SetSphereRadius` (`self.AOE`) (`self.ScaleAOE`) true)
      (`SceneComponent.SetVisibility` (`self.Widget`) false false)
      (`SceneComponent.SetVisibility` (`self.StaticMesh`) false false))
    (:`NewEnumerator3`
      (goto _label))))