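; BP_ConsumableBase is a base interactable for consumable pickups, configured from a data table row that supplies the mesh and maximum quantity.
; Interaction adds it to the player's inventory and hides it, or logs a message if the held stack is at maximum.
; Consuming removes it from inventory; both pickup and use notify the quest component.
; On BeginPlay, saved game data keeps already-picked items hidden.
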(event `self.ReceiveBeginPlay`
  (`parent.ReceiveBeginPlay`)
  (set `self.MaxQuantity` (`.Quantity_14_AC7DD1774D7D1A70B5492BB757D6C996` (break `/Game/Blueprints/Structures/FConsumable` (`self.ConsumableStructure`))))
  (`self.SyncPickedData`))

(event `self.MainBody`
  (bind _currentconsumable (`/Game/Blueprints/Common/Inventory/BP_InventoryComponent.GetCurrentConsumable` (`self.GetComponentByClass` (`GameplayStatics.GetPlayerCharacter` 0) "/Game/Blueprints/Common/Inventory/BP_InventoryComponent.BP_InventoryComponent_C") self))
  (`/Engine/EditorBlueprintResources/StandardMacros.IsValid` _currentconsumable
    (:`Is Valid`
      (if (== (`/Game/Blueprints/Common/InteractionSystem/BP_ConsumableBase.CurrentQuantity` _currentconsumable) (`self.MaxQuantity`))
        (message `/Game/Blueprints/Interfaces/BPI_InteractionSystem.UpdateLogWidget` (`GameplayStatics.GetPlayerController` 0) self "NewEnumerator3")
        (else
          (`self.PickItem`))))
    (:`Is Not Valid`
      (`self.PickItem`))))

(event `/Game/Blueprints/Interfaces/BPI_InteractionSystem.Consume`
  (params (Consumable :type "/Game/Blueprints/Common/InteractionSystem/BP_ConsumableBase Object Reference"))
  (message `/Game/Blueprints/Interfaces/BPI_InteractionSystem.RemoveFromInventory` (`self.GetComponentByClass` (`GameplayStatics.GetPlayerCharacter` 0) "/Game/Blueprints/Common/Inventory/BP_InventoryComponent.BP_InventoryComponent_C") Consumable)
  (`/Game/Blueprints/Common/QuestSystem/BP_QuestComponent.OnQuestItemIterated` (`self.GetComponentByClass` (`GameplayStatics.GetPlayerCharacter` 0) "/Game/Blueprints/Common/QuestSystem/BP_QuestComponent.BP_QuestComponent_C") "NewEnumerator4" (`GameplayStatics.GetObjectClass` self)))

(fn `PickItem`
  (message `/Game/Blueprints/Interfaces/BPI_InteractionSystem.AddToInventory` (`self.GetComponentByClass` (`GameplayStatics.GetPlayerCharacter` 0) "/Game/Blueprints/Common/Inventory/BP_InventoryComponent.BP_InventoryComponent_C") self)
  (`self.SetActorEnableCollision` false)
  (`self.SetActorHiddenInGame` self true)
  (set `self.bPicked` true)
  (`/Game/Blueprints/Common/QuestSystem/BP_QuestComponent.OnQuestItemIterated` (`self.GetComponentByClass` (`GameplayStatics.GetPlayerCharacter` 0) "/Game/Blueprints/Common/QuestSystem/BP_QuestComponent.BP_QuestComponent_C") "NewEnumerator1" (`GameplayStatics.GetObjectClass` self)))

(fn `SyncPickedData`
  (bind _gamedata (message `/Game/Blueprints/Interfaces/BPI_GameInstance.LoadGameData` (`GameplayStatics.GetGameInstance`)))
  (if (`KismetArrayLibrary.Array_Contains` (`.PickedItems_43_82C839594FDCEDF11859408A90CDF15E` (break `/Game/Blueprints/Structures/GameDataChildren/FLevelData` (`.Level_37_C2FF1CFD417204E825B165B1F75E41BE` (break `/Game/Blueprints/Structures/FGameData` _gamedata)))) (`self.ObjectName`))
    (`self.SetActorEnableCollision` false)
    (`self.SetActorHiddenInGame` self true)
    (set `self.bPicked` true)))

(fn `UserConstructionScript`
  (bind _meshscale (`self.MeshScale`))
  (bind (_datatable _rowname) (break `DataTableRowHandle` (`self.AssetData`)))
  (`parent.UserConstructionScript`)
  (bind _returnvalue (`|GetDataTableRow` _datatable _rowname)
    (:`then`
      (set `self.ConsumableStructure` _returnvalue)
      (`StaticMeshComponent.SetStaticMesh` (`self.StaticMesh`) (`.Model_17_6467E5EF4C5BB4714150B59C0AF3DF3E` (break `/Game/Blueprints/Structures/FConsumable` (`self.ConsumableStructure`))))
      (`SceneComponent.SetWorldScale3D` (`self.StaticMesh`) (`KismetMathLibrary.MakeVector` _meshscale _meshscale _meshscale)))))