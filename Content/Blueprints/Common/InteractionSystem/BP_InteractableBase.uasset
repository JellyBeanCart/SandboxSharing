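; Base Blueprint for interactable world objects with hold-to-interact, a prompt widget and stencil highlighting.
; A looping timer waits for an "Interaction"-tagged static or skeletal mesh, then configures its collision, attaches the widget and restores the saved transform by level-and-object name.
; Focus events toggle widget and stencil, while hold time fills the progress bar.
; A completed hold runs MainBody, which notifies the player's quest component, then resets the interaction.
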(event `self.ReceiveBeginPlay`
  (bind _returnvalue (`KismetSystemLibrary.K2_SetTimerDelegate` (`|CreateDelegate` :!event `CheckComponentAndProceed`) 0.2 true))
  (set `self.CheckComponentTimer` _returnvalue)
  (bind _returnvalue_2 (`GameplayStatics.GetCurrentLevelName` true))
  (set `self.ObjectName` (`KismetStringLibrary.Concat_StrStr` _returnvalue_2 "_" (`KismetSystemLibrary.GetObjectName` self))))

(event `CheckComponentAndProceed`
  (bind _output (`|GetArrayItem` (`self.GetComponentsByTag` "/Script/Engine.SkeletalMeshComponent" "Interaction")))
  (bind _output_2 (`|GetArrayItem` (`self.GetComponentsByTag` "/Script/Engine.StaticMeshComponent" "Interaction")))
  (`/Engine/EditorBlueprintResources/StandardMacros.IsValid` _output_2
    (:`Is Valid`
      (set `self.PrimitiveComponent` _output_2))
    (:`Is Not Valid`
      (`/Engine/EditorBlueprintResources/StandardMacros.IsValid` _output
        (:`Is Valid`
          (set `self.PrimitiveComponent` _output)))))
  (`KismetSystemLibrary.K2_ClearAndInvalidateTimerHandle` (`self.CheckComponentTimer`))
  (`PrimitiveComponent.SetRenderCustomDepth` (`self.PrimitiveComponent`) true)
  (`PrimitiveComponent.SetCollisionObjectType` (`self.PrimitiveComponent`) "ECC_GameTraceChannel1")
  (`SceneComponent.K2_AttachToComponent` (`self.Widget`) (`self.PrimitiveComponent`) "None" "KeepRelative" "KeepRelative" "KeepWorld" true)
  (`self.SyncTransformData`)
  (`self.SyncDone`)
  (bind _ashud_interaction (cast `/Game/GUI/HUD/HUD_Interaction` (`WidgetComponent.GetUserWidgetObject` (`self.Widget`))))
  (set `self.GUI_Interaction` _ashud_interaction))

(event `/Game/Blueprints/Interfaces/BPI_InteractionSystem.CanInteract`
  (`SceneComponent.SetVisibility` (`self.Widget`) true false)
  (message `/Game/Blueprints/Interfaces/BPI_InteractionSystem.SendInteractableInfo` (`GameplayStatics.GetPlayerCharacter` 0) self)
  (`PrimitiveComponent.SetCustomDepthStencilValue` (`self.PrimitiveComponent`) 1)
  (set `/Game/GUI/HUD/HUD_Interaction.InteractableType` (`self.InteractableType`) (`self.GUI_Interaction`)))

(event `/Game/Blueprints/Interfaces/BPI_InteractionSystem.StopInteracting`
  (`SceneComponent.SetVisibility` (`self.Widget`) false false)
  (set `self.bSuccess` false)
  (`PrimitiveComponent.SetCustomDepthStencilValue` (`self.PrimitiveComponent`) 0))

(event `/Game/Blueprints/Interfaces/BPI_InteractionSystem.StartInteracting`
  (params (InteractionTime :type "Float (single-precision)"))
  (set `self.KeyHoldTime` InteractionTime)
  (if (`self.bSuccess`)
    (`/Engine/EditorBlueprintResources/StandardMacros.DoOnce` false :!label _label
      (:`Completed`
        (`self.MainBody`)
        (message `/Game/Blueprints/Interfaces/BPI_InteractionSystem.ResetInteraction` (`GameplayStatics.GetPlayerCharacter` 0) self)
        (set `self.bSuccess` false)
        (`/Game/Blueprints/Interfaces/BPI_InteractionSystem.CanInteract`)))
    (else
      (`self.SuccessInteraction`)
      (goto _label :!via `Reset`))))

(event `SuccessInteraction`
  (bind _returnvalue (`KismetMathLibrary.FClamp` (`KismetMathLibrary.SafeDivide` (`self.KeyHoldTime`) (`self.InteractionTime`))))
  (if (`SceneComponent.IsVisible` (`self.Widget`))
    (if (< _returnvalue 1.0)
      (`/Game/GUI/HUD/HUD_Interaction.UpdateProgressBar` (`self.GUI_Interaction`) _returnvalue (- (`self.InteractionTime`) (`self.KeyHoldTime`)))
      (if (== (`self.KeyHoldTime`) 0.0)
        (`/Game/GUI/HUD/HUD_Interaction.UpdateProgressBar` (`self.GUI_Interaction`) 0.0 0.0))
      (else
        (`/Game/GUI/HUD/HUD_Interaction.UpdateProgressBar` (`self.GUI_Interaction`) 0.0 0.0)
        (set `self.bSuccess` true)))))

(event `MainBody`
  (`/Game/Blueprints/Common/QuestSystem/BP_QuestComponent.OnQuestItemInteracted` (`self.GetComponentByClass` (`GameplayStatics.GetPlayerCharacter` 0) "/Game/Blueprints/Common/QuestSystem/BP_QuestComponent.BP_QuestComponent_C") "NewEnumerator3" (`GameplayStatics.GetObjectClass` self)))

(fn `GetActiveConsumableWidget`
  (returns (GUI_Consumable :type "/Game/GUI/HUD/HUD_Consumable Object Reference"))
  (return null))

(fn `GetPieMenuWidget`
  (returns (GUI_PieMenu :type "/Game/GUI/HUD/HUD_PieMenu Object Reference"))
  (return null))

(fn `SyncTransformData`
  (locals (StoredLevelData :type "/Game/Blueprints/Structures/GameDataChildren/FLevelData Structure") (ObjectNameList :type "Array of String"))
  (bind _gamedata (message `/Game/Blueprints/Interfaces/BPI_GameInstance.LoadGameData` (`GameplayStatics.GetGameInstance`)))
  (bind _output_get (set `local.StoredLevelData` (`.Level_37_C2FF1CFD417204E825B165B1F75E41BE` (break `/Game/Blueprints/Structures/FGameData` _gamedata))))
  (bind _keys (`BlueprintMapLibrary.Map_Keys` (`.LevelsInteractiveTransform_42_73873CB14345D48B70C0ED98D04B9C10` (break `/Game/Blueprints/Structures/GameDataChildren/FLevelData` _output_get))))
  (bind _output_get_2 (set `local.ObjectNameList` _keys))
  (for _array_element _output_get_2
    (if (`KismetStringLibrary.EqualEqual_StrStr` _array_element (`self.ObjectName`))
      (`self.K2_SetActorTransform` (`BlueprintMapLibrary.Map_Find` (`.LevelsInteractiveTransform_42_73873CB14345D48B70C0ED98D04B9C10` (break `/Game/Blueprints/Structures/GameDataChildren/FLevelData` (`local.StoredLevelData`))) (`self.ObjectName`)) false true))))

(fn `UserConstructionScript`)