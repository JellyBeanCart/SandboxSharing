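; Actor component that lets the player character detect interactable objects in front of its first-person camera.
; On BeginPlay it caches the owning BP_PlayerCharacter and starts a looping timer, presumably driving LineTrace, which casts a short object-type trace along the camera's view.
; It stores the hit as LastInteractable and sends CanInteract or StopInteracting messages as the target changes.
; Mutually resetting DoOnce gates keep these messages from repeating on every trace.
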(event `self.ReceiveBeginPlay`
  (bind _asbp_player_character (cast `/Game/Blueprints/Core/BP_PlayerCharacter` (`self.GetOwner`)))
  (set `self.PlayerCharacter` _asbp_player_character)
  (bind _returnvalue (`KismetSystemLibrary.K2_SetTimerDelegate` (`|CreateDelegate` :!event `LineTrace`) 0.2 true))
  (set `self.LineTraceTimer` _returnvalue))

(event `ResetValidPrevious`
  (goto _label :!via `Reset`))

(event `LineTrace`
  (bind _fpcamera (`/Game/Blueprints/Core/BP_PlayerCharacter.FPCamera` (`self.PlayerCharacter`)))
  (bind _returnvalue (`self.K2_GetComponentLocation` _fpcamera))
  (`/Engine/EditorBlueprintResources/StandardMacros.IsValid` (`self.PlayerCharacter`)
    (:`Is Valid`
      (bind _outhit (`KismetSystemLibrary.LineTraceSingleForObjects` _returnvalue (+ _returnvalue (* (`self.GetForwardVector` _fpcamera) 200.0)) (`|MakeArray` "ObjectTypeQuery7" :!type "EObjectTypeQuery Enum")))
      (`/Engine/EditorBlueprintResources/StandardMacros.IsValid` (`self.LastInteractable`)
        (:`Is Valid`
          (bind (_bblockinghit _binitialoverlap _time _distance _location _impactpoint _normal _impactnormal _physmat _hitactor) (`GameplayStatics.BreakHitResult` _outhit))
          (if (== _hitactor (`self.LastInteractable`))
            (`/Engine/EditorBlueprintResources/StandardMacros.DoOnce` false :!label _label
              (:`Completed`
                (message `/Game/Blueprints/Interfaces/BPI_InteractionSystem.CanInteract` (`self.LastInteractable`))))
            (else
              (`/Engine/EditorBlueprintResources/StandardMacros.DoOnce` false :!label _label_2
                (:`Completed`
                  (message `/Game/Blueprints/Interfaces/BPI_InteractionSystem.StopInteracting` (`self.LastInteractable`))
                  (set `self.LastInteractable` null)))))
          (`self.ResetNull`))
        (:`Is Not Valid`
          (set `self.LastInteractable` _hitactor)
          (`/Engine/EditorBlueprintResources/StandardMacros.DoOnce` false :!label _label_3
            (:`Completed`
              (message `/Game/Blueprints/Interfaces/BPI_InteractionSystem.CanInteract` (`self.LastInteractable`))
              (`self.ResetValidNew`)
              (`self.ResetValidPrevious`))))))))

(event `ResetValidNew`
  (goto _label_2 :!via `Reset`))

(event `ResetNull`
  (goto _label_3 :!via `Reset`))