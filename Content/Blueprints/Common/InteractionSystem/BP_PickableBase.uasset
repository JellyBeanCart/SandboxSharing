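; Base interactable for physics props that the player can grab, carry and release, reporting both grab and release to the player's quest component.
; Its main interaction toggles between Grab, which requires a trace to hit the player pawn, and Release, updating the action text.
; A looping timer holds the object in front of the first-person camera through the player's PhysicsHandle.
; Release clears the timer and teleports the actor to the handle's target transform.
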(event `self.ReceiveBeginPlay`
  (`parent.ReceiveBeginPlay`)
  (add `self.SyncDone` (`|CreateDelegate` :!event `Simulation`)))

(event `Simulation`
  (`PrimitiveComponent.SetSimulatePhysics` (`self.StaticMesh`) true))

(event `self.MainBody`
  (if (`self.bResetMainBody`)
    (`self.Release`)
    (else
      (`self.Grab`))))

(event `Grab`
  (bind _outhit (`KismetSystemLibrary.LineTraceSingleForObjects` (`self.K2_GetActorLocation`) (`self.K2_GetActorLocation` (`/Game/Blueprints/FunctionLibrary/BP_FunctionLibrary.GetPlayerCharacter`)) (`|MakeArray` "ObjectTypeQuery3" :!type "EObjectTypeQuery Enum")))
  (cast `/Game/Blueprints/Core/BP_PlayerCharacter` (`.HitActor` (`GameplayStatics.BreakHitResult` _outhit)))
  (bind _returnvalue (`KismetSystemLibrary.K2_SetTimerDelegate` (`|CreateDelegate` :!event `Carry`) 0.02 true))
  (set `self.CarryTimer` _returnvalue)
  (`PhysicsHandleComponent.GrabComponentAtLocationWithRotation` (`/Game/Blueprints/Core/BP_PlayerCharacter.PhysicsHandle` (`/Game/Blueprints/FunctionLibrary/BP_FunctionLibrary.GetPlayerCharacter`)) (`self.StaticMesh`) "None" (`self.GetActorBounds` false) (`SceneComponent.RelativeRotation` (`self.StaticMesh`)))
  (set `self.bResetMainBody` true)
  (`/Game/GUI/HUD/HUD_Interaction.UpdateActionText` (`self.GUI_Interaction`) "Release")
  (`/Game/Blueprints/Common/QuestSystem/BP_QuestComponent.OnQuestItemInteracted` (`self.GetComponentByClass` (`GameplayStatics.GetPlayerCharacter` 0) "/Game/Blueprints/Common/QuestSystem/BP_QuestComponent.BP_QuestComponent_C") "NewEnumerator5" (`GameplayStatics.GetObjectClass` self)))

(event `Carry`
  (bind _fpcamera (`/Game/Blueprints/Core/BP_PlayerCharacter.FPCamera` (`/Game/Blueprints/FunctionLibrary/BP_FunctionLibrary.GetPlayerCharacter`)))
  (`PhysicsHandleComponent.SetTargetLocationAndRotation` (`/Game/Blueprints/Core/BP_PlayerCharacter.PhysicsHandle` (`/Game/Blueprints/FunctionLibrary/BP_FunctionLibrary.GetPlayerCharacter`)) (+ (`SceneComponent.K2_GetComponentLocation` _fpcamera) (* (`SceneComponent.GetForwardVector` _fpcamera) 100.0)) (`self.K2_GetActorRotation` (`/Game/Blueprints/FunctionLibrary/BP_FunctionLibrary.GetPlayerCharacter`))))

(event `/Game/Blueprints/Interfaces/BPI_InteractionSystem.StopInteracting`
  (`parent.StopInteracting`)
  (`self.Release`))

(event `Release`
  (bind (_targetlocation _targetrotation) (`PhysicsHandleComponent.GetTargetLocationAndRotation` (`/Game/Blueprints/Core/BP_PlayerCharacter.PhysicsHandle` (`/Game/Blueprints/FunctionLibrary/BP_FunctionLibrary.GetPlayerCharacter`))))
  (`PhysicsHandleComponent.ReleaseComponent` (`/Game/Blueprints/Core/BP_PlayerCharacter.PhysicsHandle` (`/Game/Blueprints/FunctionLibrary/BP_FunctionLibrary.GetPlayerCharacter`)))
  (`KismetSystemLibrary.K2_ClearAndInvalidateTimerHandle` (`self.CarryTimer`))
  (set `self.bResetMainBody` false)
  (`/Game/GUI/HUD/HUD_Interaction.UpdateActionText` (`self.GUI_Interaction`) "Grab")
  (`self.K2_SetActorLocationAndRotation` _targetlocation _targetrotation false true)
  (`/Game/Blueprints/Common/QuestSystem/BP_QuestComponent.OnQuestItemInteracted` (`self.GetComponentByClass` (`GameplayStatics.GetPlayerCharacter` 0) "/Game/Blueprints/Common/QuestSystem/BP_QuestComponent.BP_QuestComponent_C") "NewEnumerator6" (`GameplayStatics.GetObjectClass` self)))

(fn `UserConstructionScript`
  (`parent.UserConstructionScript`)
  (`SceneComponent.SetRelativeScale3D` (`self.StaticMesh`) (* (1.0 1.0 1.0) (`self.ModelScale`))))