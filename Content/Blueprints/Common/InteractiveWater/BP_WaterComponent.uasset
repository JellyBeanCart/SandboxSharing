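; Actor component that makes its owner's static mesh float and splash in BP_InteractiveWater.
; Each tick, a short downward trace from the mesh's bounds finds water, applying splats while the mesh moves and isn't submerged.
; A second trace over the water's buoyancy height drives an acceleration along the hit normal, weakening with distance, and raises damping.
; Damping resets when no water is hit; a looping timer supports the movement check.
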(event `SavePreviousLocation`
  (set `self.PreviousLocation` (`self.K2_GetComponentLocation` (`self.AffectedMesh`))))

(event `self.ReceiveBeginPlay`
  (set `self.AffectedMesh` (`Actor.GetComponentByClass` (`self.GetOwner`) "/Script/Engine.StaticMeshComponent"))
  (`KismetSystemLibrary.K2_SetTimerDelegate` (`|CreateDelegate` :!event `SavePreviousLocation`) 1.0 true))

(event `self.ReceiveTick`
  (params (DeltaSeconds :type "Float (single-precision)"))
  (bind (_start _end) (`self.ComputeTrace` 1.0))
  (bind (_start_2 _end_2) (`self.ComputeTrace` (`/Game/Blueprints/Common/InteractiveWater/BP_InteractiveWater.BuoyancyHeight` (`self.InteractiveWater`))))
  (`/Engine/EditorBlueprintResources/StandardMacros.IsValid` (`self.GetOwner`)
    (:`Is Valid`
      (bind (_outhit _returnvalue) (`KismetSystemLibrary.LineTraceSingleForObjects` _start _end (`|MakeArray` "ObjectTypeQuery8" :!type "EObjectTypeQuery Enum")))
      (if _returnvalue
        (set `self.WaterHit` _outhit)
        (bind _asbp_interactive_water (cast `/Game/Blueprints/Common/InteractiveWater/BP_InteractiveWater` (`.HitActor` (`GameplayStatics.BreakHitResult` (`self.WaterHit`)))))
        (set `self.InteractiveWater` _asbp_interactive_water)
        (if (not (`self.IsUnderWater`))
          (if (not (== (`self.K2_GetComponentLocation` (`self.AffectedMesh`)) (`self.PreviousLocation`) :`ErrorTolerance` 5.0))
            (`/Game/Blueprints/Common/InteractiveWater/BP_InteractiveWater.ApplyLocalSplat` (`self.InteractiveWater`) (`self.K2_GetComponentLocation` (`self.AffectedMesh`)) (`self.ImpactSize`))))
        (bind (_outhit_2 _returnvalue_2) (`KismetSystemLibrary.LineTraceSingleForObjects` _start_2 _end_2 (`|MakeArray` "ObjectTypeQuery9" :!type "EObjectTypeQuery Enum")))
        (if _returnvalue_2
          (set `self.BuoyancyHit` _outhit_2)
          (`PrimitiveComponent.AddForce` (`self.AffectedMesh`) (`self.ComputeBuoyancyEffect`) "None" true)
          (`PrimitiveComponent.SetLinearDamping` (`self.AffectedMesh`) (`self.LinearDamping`))
          (`PrimitiveComponent.SetAngularDamping` (`self.AffectedMesh`) (`self.AngularDamping`)))
        (else
          (`PrimitiveComponent.SetLinearDamping` (`self.AffectedMesh`) 0.01)
          (`PrimitiveComponent.SetAngularDamping` (`self.AffectedMesh`) 0.0))))))

(fn `ComputeBuoyancyEffect`
  (returns (Force :type "Vector Structure"))
  (return (* (`.ImpactNormal` (`GameplayStatics.BreakHitResult` (`self.BuoyancyHit`))) (`KismetMathLibrary.Lerp` (`self.BuoyancyForce`) (* (`self.BuoyancyForce`) 0.35) (/ (`KismetMathLibrary.VSize` (- (`.Location` (`GameplayStatics.BreakHitResult` (`self.BuoyancyHit`))) (`self.K2_GetComponentLocation` (`self.AffectedMesh`)))) (`/Game/Blueprints/Common/InteractiveWater/BP_InteractiveWater.BuoyancyHeight` (`self.InteractiveWater`)))))))

(fn `ComputeTrace`
  (params (Distance :type "Float (double-precision)"))
  (returns (Start :type "Vector Structure") (End :type "Vector Structure"))
  (bind (_origin _boxextent) (`KismetSystemLibrary.GetComponentBounds` (`self.AffectedMesh`)))
  (bind _returnvalue (`KismetMathLibrary.MakeVector` (.x _origin) (.y _origin) (- (.z _origin) (.z _boxextent))))
  (return _returnvalue (+ _returnvalue (* (0.0 0.0 -1.0) (`local.Distance`)))))

(fn `IsUnderWater`
  (returns (Value :type Boolean))
  (bind (_origin _boxextent) (`KismetSystemLibrary.GetComponentBounds` (`self.AffectedMesh`)))
  (bind (_origin_2 _boxextent_2) (`KismetSystemLibrary.GetComponentBounds` (`/Game/Blueprints/Common/InteractiveWater/BP_InteractiveWater.Box` (`self.InteractiveWater`))))
  (return (`KismetMathLibrary.IsPointInBox` (`KismetMathLibrary.MakeVector` (.x _origin) (.y _origin) (+ (.z _origin) (.z _boxextent))) _origin_2 _boxextent_2)))