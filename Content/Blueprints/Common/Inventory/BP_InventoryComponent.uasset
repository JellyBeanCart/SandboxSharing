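; Inventory component that tracks the player's consumables, keeping one actor and a quantity per class in parallel class and object arrays.
; A looping timer waits for the pie menu and active consumable widgets, then restores saved items as hidden, collision-free actors.
; Add and remove events, ignored until restoration finishes, adjust quantities and update the UI through controller messages.
; Restoration and removal also sync the active consumable with the player character.
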(event `self.ReceiveBeginPlay`
  (bind _returnvalue (`KismetSystemLibrary.K2_SetTimerDelegate` (`|CreateDelegate` :!event `CheckInventoryWidgets`) 0.2 true))
  (set `self.CheckInventoryWidgetsTimer` _returnvalue))

(event `CheckInventoryWidgets`
  (bind _gui_piemenu (message `/Game/Blueprints/Interfaces/BPI_InteractionSystem.GetPieMenuWidget` (`GameplayStatics.GetPlayerController` 0)))
  (`/Engine/EditorBlueprintResources/StandardMacros.IsValid` _gui_piemenu
    (:`Is Valid`
      (bind _gui_consumable (message `/Game/Blueprints/Interfaces/BPI_InteractionSystem.GetActiveConsumableWidget` (`GameplayStatics.GetPlayerController` 0)))
      (`/Engine/EditorBlueprintResources/StandardMacros.IsValid` _gui_consumable
        (:`Is Valid`
          (`KismetSystemLibrary.K2_ClearAndInvalidateTimerHandle` (`self.CheckInventoryWidgetsTimer`))
          (`self.RestoreInventory`)
          (set `self.bInventoryReady` true))))))

(event `/Game/Blueprints/Interfaces/BPI_InteractionSystem.AddToInventory`
  (params (Consumable :type "/Game/Blueprints/Common/InteractionSystem/BP_ConsumableBase Object Reference"))
  (if (`self.bInventoryReady`)
    (set `self.LastConsumable` Consumable)
    (if (`KismetArrayLibrary.Array_Contains` (`self.ConsumableClassList`) (`GameplayStatics.GetObjectClass` (`self.LastConsumable`)))
      (bind _currentconsumable (`self.GetCurrentConsumable` (`self.LastConsumable`)))
      (set `self.LastConsumable` _currentconsumable)
      (else
        (`KismetArrayLibrary.Array_AddUnique` (`self.ConsumableClassList`) (`GameplayStatics.GetObjectClass` (`self.LastConsumable`)))
        (`KismetArrayLibrary.Array_AddUnique` (`self.ConsumableObjectList`) (`self.LastConsumable`))))
    (set `/Game/Blueprints/Common/InteractionSystem/BP_ConsumableBase.CurrentQuantity` (+ (`/Game/Blueprints/Common/InteractionSystem/BP_ConsumableBase.CurrentQuantity` (`self.LastConsumable`)) 1) (`self.LastConsumable`))
    (message `/Game/Blueprints/Interfaces/BPI_InteractionSystem.UpdatePieMenu` (`GameplayStatics.GetPlayerController` 0) (`self.LastConsumable`))
    (message `/Game/Blueprints/Interfaces/BPI_InteractionSystem.UpdateLogWidget` (`GameplayStatics.GetPlayerController` 0) (`self.LastConsumable`) "NewEnumerator1")
    (if (== (`GameplayStatics.GetObjectClass` (`self.LastConsumable`)) (`GameplayStatics.GetObjectClass` (`self.ActiveConsumable`)))
      (message `/Game/Blueprints/Interfaces/BPI_InteractionSystem.UpdateConsumableWidget` (`GameplayStatics.GetPlayerController` 0) (`self.LastConsumable`)))))

(event `/Game/Blueprints/Interfaces/BPI_InteractionSystem.SetActiveConsumable`
  (params (Consumable :type "/Game/Blueprints/Common/InteractionSystem/BP_ConsumableBase Object Reference"))
  (set `self.ActiveConsumable` Consumable))

(event `/Game/Blueprints/Interfaces/BPI_InteractionSystem.RemoveFromInventory`
  (params (Consumable :type "/Game/Blueprints/Common/InteractionSystem/BP_ConsumableBase Object Reference"))
  (if (`self.bInventoryReady`)
    (set `self.LastConsumable` Consumable)
    (message `/Game/Blueprints/Interfaces/BPI_InteractionSystem.UpdateLogWidget` (`GameplayStatics.GetPlayerController` 0) (`self.LastConsumable`) "NewEnumerator2")
    (bind _output_get (set `/Game/Blueprints/Common/InteractionSystem/BP_ConsumableBase.CurrentQuantity` (- (`/Game/Blueprints/Common/InteractionSystem/BP_ConsumableBase.CurrentQuantity` (`self.LastConsumable`)) 1) (`self.LastConsumable`)))
    (if (== _output_get 0)
      (message `/Game/Blueprints/Interfaces/BPI_InteractionSystem.SetActiveConsumable` (`GameplayStatics.GetPlayerCharacter` 0) null)
      (message `/Game/Blueprints/Interfaces/BPI_InteractionSystem.UpdatePieMenu` (`GameplayStatics.GetPlayerController` 0) null)
      (message `/Game/Blueprints/Interfaces/BPI_InteractionSystem.UpdateConsumableWidget` (`GameplayStatics.GetPlayerController` 0) null)
      (message `/Game/Blueprints/Interfaces/BPI_InteractionSystem.UpdateLogWidget` (`GameplayStatics.GetPlayerController` 0) (`self.LastConsumable`) "NewEnumerator4")
      (else
        (message `/Game/Blueprints/Interfaces/BPI_InteractionSystem.SetActiveConsumable` (`GameplayStatics.GetPlayerCharacter` 0) (`self.LastConsumable`))
        (message `/Game/Blueprints/Interfaces/BPI_InteractionSystem.UpdatePieMenu` (`GameplayStatics.GetPlayerController` 0) (`self.LastConsumable`))
        (message `/Game/Blueprints/Interfaces/BPI_InteractionSystem.UpdateConsumableWidget` (`GameplayStatics.GetPlayerController` 0) (`self.LastConsumable`))))))

(fn `GetActiveConsumableWidget`
  (returns (GUI_Consumable :type "/Game/GUI/HUD/HUD_Consumable Object Reference"))
  (return null))

(fn `GetCurrentConsumable`
  (params (Consumable :type "/Game/Blueprints/Common/InteractionSystem/BP_ConsumableBase Object Reference"))
  (returns (CurrentConsumable :type "/Game/Blueprints/Common/InteractionSystem/BP_ConsumableBase Object Reference"))
  (return (`|GetArrayItem` (`self.ConsumableObjectList`) (`KismetArrayLibrary.Array_Find` (`self.ConsumableClassList`) (`GameplayStatics.GetObjectClass` (`local.Consumable`))))))

(fn `GetPieMenuWidget`
  (returns (GUI_PieMenu :type "/Game/GUI/HUD/HUD_PieMenu Object Reference"))
  (return null))

(fn `RestoreInventory`
  (locals (BasicTransform :type "Transform Structure") (StoredPlayerData :type "/Game/Blueprints/Structures/GameDataChildren/FPlayerData Structure"))
  (bind _gamedata (message `/Game/Blueprints/Interfaces/BPI_GameInstance.LoadGameData` (`GameplayStatics.GetGameInstance`)))
  (bind _output_get (set `local.StoredPlayerData` (`.Player_34_DD80CB954E9A40AF1BD1338114B3921E` (break `/Game/Blueprints/Structures/FGameData` _gamedata))))
  (bind _keys (`BlueprintMapLibrary.Map_Keys` (`.Inventory_10_88C2D6B445CB8D15CEA9928E71CDF194` (break `/Game/Blueprints/Structures/GameDataChildren/FPlayerData` _output_get))))
  (bind _output_get_2 (set `self.ConsumableClassList` _keys))
  (for _array_element _output_get_2
    (bind (_value _returnvalue) (`BlueprintMapLibrary.Map_Find` (`.Inventory_10_88C2D6B445CB8D15CEA9928E71CDF194` (break `/Game/Blueprints/Structures/GameDataChildren/FPlayerData` (`local.StoredPlayerData`))) _array_element))
    (if _returnvalue
      (bind _returnvalue_2 (`|SpawnActorFromClass` _array_element (`local.BasicTransform`) "AlwaysSpawn" "OverrideRootScale" null null))
      (`KismetArrayLibrary.Array_AddUnique` (`self.ConsumableObjectList`) _returnvalue_2)
      (set `/Game/Blueprints/Common/InteractionSystem/BP_ConsumableBase.CurrentQuantity` _value _returnvalue_2)
      (`Actor.SetActorEnableCollision` _returnvalue_2 false)
      (`Actor.SetActorHiddenInGame` _returnvalue_2 true)
      (message `/Game/Blueprints/Interfaces/BPI_InteractionSystem.UpdatePieMenu` (`GameplayStatics.GetPlayerController` 0) _returnvalue_2)
      (if (== (`GameplayStatics.GetObjectClass` _returnvalue_2) (`.Selected_13_0A75195E4236911BE5AB47AD247B7FDA` (break `/Game/Blueprints/Structures/GameDataChildren/FPlayerData` (`local.StoredPlayerData`))))
        (message `/Game/Blueprints/Interfaces/BPI_InteractionSystem.UpdateConsumableWidget` (`GameplayStatics.GetPlayerController` 0) _returnvalue_2)
        (message `/Game/Blueprints/Interfaces/BPI_InteractionSystem.SetActiveConsumable` (`GameplayStatics.GetPlayerCharacter` 0) _returnvalue_2)))))