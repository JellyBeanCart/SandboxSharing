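; Map marker actor that shows an icon plane on the player's minimap and map, configured from a data table row or as a Location type that expires when the player overlaps it.
; A timer waits for the player, then registers the plane in their map show list and requests an edge marker widget.
; A looping update rotates the plane with player yaw in minimap mode and hides it beyond minimap range.
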(event `CheckPlayerAndProceed`
  (`/Engine/EditorBlueprintResources/StandardMacros.IsValid` (`/Game/Blueprints/FunctionLibrary/BP_FunctionLibrary.GetPlayerCharacter`)
    (:`Is Valid`
      (`KismetSystemLibrary.K2_ClearAndInvalidateTimerHandle` (`self.CheckPlayerTimer`))
      (message `/Game/Blueprints/Interfaces/BPI_PlayerCharacter.UpdateMapShowList` (`GameplayStatics.GetPlayerCharacter` 0) (`self.MarkerPlane`))
      (bind _minimapsizeinunits (message `/Game/Blueprints/Interfaces/BPI_PlayerCharacter.GetMinimapData` (`GameplayStatics.GetPlayerCharacter` 0)))
      (set `self.MinimapSizeInUnits` _minimapsizeinunits)
      (message `/Game/Blueprints/Interfaces/BPI_PlayerCharacter.CreateMapEdgeMarkerWidget` (`GameplayStatics.GetPlayerController` 0) (`self.MarkerStructure`) (`self.K2_GetActorLocation`) (`self.MinimapSizeInUnits`) self)
      (bind _returnvalue (`KismetSystemLibrary.K2_SetTimerDelegate` (`|CreateDelegate` :!event `UpdateVisualFeedback`) 0.04 true))
      (set `self.VisualFeedbackTimer` _returnvalue))))

(event `self.ReceiveBeginPlay`
  (`self.UnpackDataAndProceed`)
  (bind _returnvalue (`PrimitiveComponent.CreateDynamicMaterialInstance` (`self.MarkerPlane`) 0 "/Game/GUI/Materials/M_CommonMarker.M_CommonMarker" "None"))
  (set `self.MID_CommonMarker` _returnvalue)
  (`MaterialInstanceDynamic.SetTextureParameterValue` (`self.MID_CommonMarker`) "Texture" (`.Texture_6_19DB76BB486FD45FFAE88E96B72EAF4D` (break `/Game/Blueprints/Structures/FCommonMarker` (`self.MarkerStructure`))))
  (bind _returnvalue_2 (`KismetSystemLibrary.K2_SetTimerDelegate` (`|CreateDelegate` :!event `CheckPlayerAndProceed`) 0.2 true))
  (set `self.CheckPlayerTimer` _returnvalue_2))

(event `UpdateVisualFeedback`
  (bind (_returnvalue_roll _returnvalue_pitch _returnvalue_yaw) (`KismetMathLibrary.BreakRotator` (`self.K2_GetActorRotation` (`GameplayStatics.GetPlayerCharacter` 0))))
  (bind (_minimapsizeinunits _bminimap) (message `/Game/Blueprints/Interfaces/BPI_PlayerCharacter.GetMinimapData` (`GameplayStatics.GetPlayerCharacter` 0)))
  (set `self.bMinimap` _bminimap)
  (if (not (`self.bMinimap`))
    (`SceneComponent.K2_SetRelativeRotation` (`self.MarkerPlane`) (struct :`Yaw` 90.0) false false)
    (`SceneComponent.SetVisibility` (`self.MarkerPlane`) true false)
    (else
      (`SceneComponent.K2_SetRelativeRotation` (`self.MarkerPlane`) (`KismetMathLibrary.MakeRotator` 0.0 0.0 (+ _returnvalue_yaw 90.0)) false false)
      (bind _boutsideminimaprange (`self.UpdateVisibility`))
      (if _boutsideminimaprange
        (`SceneComponent.SetVisibility` (`self.MarkerPlane`) false false)
        (else
          (`SceneComponent.SetVisibility` (`self.MarkerPlane`) true false))))))

(event `self.Box.OnComponentBeginOverlap`
  (params (OverlappedComponent :type "PrimitiveComponent Object Reference") (OtherActor :type "Actor Object Reference") (OtherComp :type "PrimitiveComponent Object Reference") (OtherBodyIndex :type Integer) (bFromSweep :type Boolean) (SweepResult :type "HitResult Structure (by ref)"))
  (cast `/Game/Blueprints/Core/BP_PlayerCharacter` OtherActor)
  (`self.DestroyMarker`))

(fn `DestroyMarker`
  (`self.SetLifeSpan` 0.2))

(fn `UnpackDataAndProceed`
  (bind (_returnvalue_x _returnvalue_y) (`KismetMathLibrary.BreakVector` (`self.K2_GetActorLocation`)))
  (bind (_datatable _rowname) (break `DataTableRowHandle` (`self.MarkerData`)))
  (bind (_size_x _size_y) (`KismetMathLibrary.BreakVector2D` (break `/Game/Blueprints/Structures/FCommonMarker` (`self.MarkerStructure`))))
  (switch `/Game/Blueprints/Enumerations/EMarkerType` (`self.MarkerType`)
    (:`NewEnumerator1`
      (bind _returnvalue (`|GetDataTableRow` _datatable _rowname)
        (:`then`
          (set `self.MarkerStructure` _returnvalue))))
    (:`NewEnumerator2`
      (set `PrimitiveComponent.bGenerateOverlapEvents` true (`self.Box`))))
  (`self.K2_SetActorLocation` (`KismetMathLibrary.MakeVector` _returnvalue_x _returnvalue_y))
  (`SceneComponent.K2_SetRelativeLocation` (`self.MarkerPlane`) (`KismetMathLibrary.MakeVector` 0.0 0.0 (`.Offset_14_8AD2F03141AFAB83689394AAB3F2C846` (break `/Game/Blueprints/Structures/FCommonMarker` (`self.MarkerStructure`)))) false false)
  (`SceneComponent.SetRelativeScale3D` (`self.MarkerPlane`) (`KismetMathLibrary.MakeVector` _size_x _size_y)))

(fn `UpdateVisibility`
  (returns (bOutsideMinimapRange :type Boolean))
  (bind (_returnvalue_x _returnvalue_y) (`KismetMathLibrary.BreakVector` (`self.K2_GetActorLocation`)))
  (bind (_returnvalue_x_2 _returnvalue_y_2) (`KismetMathLibrary.BreakVector` (`self.K2_GetActorLocation` (`Controller.GetViewTarget` (`GameplayStatics.GetPlayerController` 0)))))
  (return (> (/ (`KismetMathLibrary.VSize2D` (`KismetMathLibrary.MakeVector2D` (- _returnvalue_x_2 _returnvalue_x) (- _returnvalue_y_2 _returnvalue_y))) (`.MapSizeInKm` (`/Game/Blueprints/FunctionLibrary/BP_FunctionLibrary.GetMapCaptureSize`))) (`self.MinimapSizeInUnits`))))

(fn `UserConstructionScript`
  (`self.UnpackDataAndProceed`))