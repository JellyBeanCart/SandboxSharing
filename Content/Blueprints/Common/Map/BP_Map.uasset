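; BP_Map is a scene-capture actor that renders the minimap and world map into render targets created at BeginPlay.
; UpdateMapStatus switches which capture renders every frame: minimap mode runs a looping timer, presumably for MinimapTracking, which matches owner XY and yaw.
; World-map mode stops that timer and repositions the actor using half the world origin location.
; UpdateMapShowList adds components to both captures' show-only lists.
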(event `self.ReceiveBeginPlay`
  (bind _minimapsize (`self.MinimapSize`))
  (bind _worldmapsize (`self.WorldMapSize`))
  (bind _returnvalue (`KismetRenderingLibrary.CreateRenderTarget2D` _minimapsize _minimapsize "RTF_RGBA8"))
  (bind _output_get (set `self.RT_Minimap` _returnvalue))
  (set `SceneCaptureComponent2D.TextureTarget` _output_get (`self.MinimapComponent`))
  (set `SceneCaptureComponent2D.OrthoWidth` (* (`self.MinimapZoom`) (`/Game/Blueprints/FunctionLibrary/BP_FunctionLibrary.GetMapCaptureSize`)) (`self.MinimapComponent`))
  (bind _returnvalue_2 (`KismetRenderingLibrary.CreateRenderTarget2D` _worldmapsize _worldmapsize "RTF_RGBA8"))
  (bind _output_get_2 (set `self.RT_WorldMap` _returnvalue_2))
  (set `SceneCaptureComponent2D.TextureTarget` _output_get_2 (`self.WorldMapComponent`))
  (set `SceneCaptureComponent2D.OrthoWidth` (`/Game/Blueprints/FunctionLibrary/BP_FunctionLibrary.GetMapCaptureSize`) (`self.WorldMapComponent`))
  (`self.UpdateMapStatus` true))

(event `self.ReceiveDestroyed`
  (`KismetRenderingLibrary.ClearRenderTarget2D` (`self.RT_Minimap`))
  (`KismetRenderingLibrary.ClearRenderTarget2D` (`self.RT_WorldMap`))
  (`KismetSystemLibrary.K2_ClearAndInvalidateTimerHandle` (`self.TrackingTimer`)))

(fn `DestroyMap`
  (`self.K2_DestroyActor`))

(fn `MinimapTracking`
  (bind _returnvalue (`self.GetOwner`))
  (bind (_returnvalue_x _returnvalue_y _returnvalue_z) (`KismetMathLibrary.BreakVector` (`self.K2_GetActorLocation`)))
  (bind (_returnvalue_roll _returnvalue_pitch _returnvalue_yaw) (`KismetMathLibrary.BreakRotator` (`self.K2_GetActorRotation` _returnvalue)))
  (bind (_returnvalue_x_2 _returnvalue_y_2) (`KismetMathLibrary.BreakVector` (`self.K2_GetActorLocation` _returnvalue)))
  (`self.K2_SetActorLocationAndRotation` (`KismetMathLibrary.MakeVector` _returnvalue_x_2 _returnvalue_y_2 _returnvalue_z) (`KismetMathLibrary.MakeRotator` 0.0 0.0 _returnvalue_yaw)))

(fn `UpdateMapShowList`
  (params (ShowComponent :type "PrimitiveComponent Object Reference"))
  (`SceneCaptureComponent.ShowOnlyComponent` (`self.MinimapComponent`) (`local.ShowComponent`))
  (`SceneCaptureComponent.ShowOnlyComponent` (`self.WorldMapComponent`) (`local.ShowComponent`)))

(fn `UpdateMapStatus`
  (params (bMinimap :type Boolean))
  (bind (_returnvalue_x _returnvalue_y) (break `IntVector` (`GameplayStatics.GetWorldOriginLocation`)))
  (bind (_returnvalue_x_2 _returnvalue_y_2 _returnvalue_z) (`KismetMathLibrary.BreakVector` (`self.K2_GetActorLocation`)))
  (if bMinimap
    (bind _returnvalue (`KismetSystemLibrary.K2_SetTimerDelegate` (`|CreateDelegate` :!event `MinimapTracking`) 0.04 true))
    (set `self.TrackingTimer` _returnvalue)
    (set `SceneCaptureComponent.bCaptureEveryFrame` true (`self.MinimapComponent`))
    (set `SceneCaptureComponent.bCaptureEveryFrame` false (`self.WorldMapComponent`))
    (else
      (`self.K2_SetActorLocationAndRotation` (`KismetMathLibrary.MakeVector` (/ (`KismetMathLibrary.Conv_IntToDouble` _returnvalue_x) 2.0) (/ (`KismetMathLibrary.Conv_IntToDouble` _returnvalue_y) 2.0) _returnvalue_z) (`KismetMathLibrary.MakeRotator` 0.0))
      (`KismetSystemLibrary.K2_ClearAndInvalidateTimerHandle` (`self.TrackingTimer`))
      (set `SceneCaptureComponent.bCaptureEveryFrame` false (`self.MinimapComponent`))
      (set `SceneCaptureComponent.bCaptureEveryFrame` true (`self.WorldMapComponent`)))))

(fn `UserConstructionScript`)