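; Map actor that captures a top-down world texture and draws player routes for the minimap.
; Construction sizes the camera and projection plane to the world, optionally exporting an orthographic capture of "Capture"-tagged actors as PNG.
; At play, it textures the plane and registers it with the player's map show list.
; MakeRoute toggles a destination marker; a looping timer rebuilds navigation-path spline meshes far below ground for the minimap.
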(event `CheckPlayerAndProceed`
  (`/Engine/EditorBlueprintResources/StandardMacros.IsValid` (`/Game/Blueprints/FunctionLibrary/BP_FunctionLibrary.GetPlayerCharacter`)
    (:`Is Valid`
      (`KismetSystemLibrary.K2_ClearAndInvalidateTimerHandle` (`self.CheckPlayerTimer`))
      (message `/Game/Blueprints/Interfaces/BPI_PlayerCharacter.UpdateMapShowList` (`GameplayStatics.GetPlayerCharacter` 0) (`self.ProjectionPlane`)))))

(event `self.ReceiveBeginPlay`
  (bind _returnvalue (`PrimitiveComponent.CreateDynamicMaterialInstance` (`self.ProjectionPlane`) 0 "/Game/GUI/Materials/M_MapProjection.M_MapProjection" "None"))
  (set `self.MID_MapProjection` _returnvalue)
  (`MaterialInstanceDynamic.SetTextureParameterValue` (`self.MID_MapProjection`) "Texture" (`self.MapTexture`))
  (bind _returnvalue_2 (`KismetSystemLibrary.K2_SetTimerDelegate` (`|CreateDelegate` :!event `CheckPlayerAndProceed`) 0.2 true))
  (set `self.CheckPlayerTimer` _returnvalue_2))

(event `DrawRoute`
  (bind (_finallocation_x _finallocation_y) (`KismetMathLibrary.BreakVector` (`self.FinalLocation`)))
  (bind (_returnvalue_x _returnvalue_y) (`KismetMathLibrary.BreakVector` (`self.K2_GetActorLocation` (`GameplayStatics.GetPlayerCharacter` 0))))
  (`/Engine/EditorBlueprintResources/StandardMacros.IsValid` (`self.RoutePin`)
    (:`Is Valid`
      (for _array_element (`self.SplineMeshList`)
        (`ActorComponent.K2_DestroyComponent` _array_element))
      (`KismetArrayLibrary.Array_Clear` (`self.SplineMeshList`))
      (bind _returnvalue (`NavigationSystemV1.FindPathToLocationSynchronously` (`KismetMathLibrary.MakeVector` _returnvalue_x _returnvalue_y) (`KismetMathLibrary.MakeVector` _finallocation_x _finallocation_y) null null))
      (bind _output_get (set `self.Route` (`NavigationPath.PathPoints` _returnvalue)))
      (`SplineComponent.SetSplinePoints` (`self.SplineComponent`) _output_get "World" true)
      (for _index (range (`SplineComponent.GetNumberOfSplineSegments` (`self.SplineComponent`)))
        (set `self.SplineSegmentIndex` _index)
        (bind _returnvalue_2 (`AddComponent|NODE_AddSplineMeshComponent-3` :`RelativeTransform` (`KismetMathLibrary.MakeTransform` (0.0 0.0 -150000.0))))
        (`KismetArrayLibrary.Array_Add` (`self.SplineMeshList`) _returnvalue_2)
        (`SplineMeshComponent.SetStartAndEnd` _returnvalue_2 (`SplineComponent.GetLocationAtSplinePoint` (`self.SplineComponent`) (`self.SplineSegmentIndex`) "Local") (0.0 0.0 0.0) (`SplineComponent.GetLocationAtSplinePoint` (`self.SplineComponent`) (+ (`self.SplineSegmentIndex`) 1) "Local") (0.0 0.0 0.0) true))
      (bind (_minimapsizeinunits _bminimap _minimapreference) (message `/Game/Blueprints/Interfaces/BPI_PlayerCharacter.GetMinimapData` (`GameplayStatics.GetPlayerCharacter` 0)))
      (for _array_element_2 (`self.SplineMeshList`)
        (`/Game/Blueprints/Common/Map/BP_Map.UpdateMapShowList` _minimapreference _array_element_2)))
    (:`Is Not Valid`
      (`KismetSystemLibrary.K2_ClearAndInvalidateTimerHandle` (`self.DrawRouteTimer`))
      (for _array_element_3 (`self.SplineMeshList`)
        (`ActorComponent.K2_DestroyComponent` _array_element_3))
      (`KismetArrayLibrary.Array_Clear` (`self.SplineMeshList`)))))

(fn `MakeMapCapture`
  (locals (RT_MapCapture :type "TextureRenderTarget2D Object Reference"))
  (bind _capturesize (`self.CaptureSize`))
  (bind _returnvalue (`KismetRenderingLibrary.CreateRenderTarget2D` _capturesize _capturesize "RTF_RGBA8"))
  (bind _output_get (set `local.RT_MapCapture` _returnvalue))
  (set `SceneCaptureComponent2D.TextureTarget` _output_get (`self.SceneCapture`))
  (set `SceneCaptureComponent2D.OrthoWidth` (`self.WorldSizeInUnits`) (`self.SceneCapture`))
  (bind _outactors (`GameplayStatics.GetAllActorsWithTag` "Capture"))
  (set `SceneCaptureComponent.ShowOnlyActors` _outactors (`self.SceneCapture`))
  (`SceneCaptureComponent2D.CaptureScene` (`self.SceneCapture`))
  (if (`KismetStringLibrary.NotEqual_StrStr` (`self.TextureName`))
    (`KismetRenderingLibrary.ExportRenderTarget` (`local.RT_MapCapture`) (`KismetStringLibrary.Concat_StrStr` (`KismetSystemLibrary.GetProjectContentDirectory`) "/Maps/MapCapture") (`KismetStringLibrary.Concat_StrStr` "T_" (`self.TextureName`) ".png"))
    (set `self.bCapture` false)))

(fn `MakeRoute`
  (params (FinalLocation :type "Vector Structure") (LocationPin :type "Actor Object Reference"))
  (set `self.FinalLocation` FinalLocation)
  (bind _output_get (set `self.LocationPin` LocationPin))
  (bind _asbp_common_marker (cast `/Game/Blueprints/Common/Map/BP_CommonMarker` _output_get)
    (:`then`
      (if (`|EnumEquality` (`/Game/Blueprints/Common/Map/BP_CommonMarker.MarkerType` _asbp_common_marker) "NewEnumerator2")
        (if (== (`self.RoutePin`) (`local.LocationPin`))
          (`/Game/Blueprints/Common/Map/BP_CommonMarker.DestroyMarker` (`self.RoutePin`))
          (`ActorComponent.K2_DestroyComponent` (`self.SplineComponent`))
          (for _array_element (`self.SplineMeshList`)
            (`ActorComponent.K2_DestroyComponent` _array_element))
          (`KismetArrayLibrary.Array_Clear` (`self.SplineMeshList`))
          (`KismetSystemLibrary.K2_ClearAndInvalidateTimerHandle` (`self.DrawRouteTimer`)))))
    (:`CastFailed`
      (`/Engine/EditorBlueprintResources/StandardMacros.IsValid` (`self.RoutePin`)
        (:`Is Valid`
          (`/Game/Blueprints/Common/Map/BP_CommonMarker.DestroyMarker` (`self.RoutePin`))
          (for _array_element_2 (`self.SplineMeshList`)
            (`ActorComponent.K2_DestroyComponent` _array_element_2))
          (`KismetArrayLibrary.Array_Clear` (`self.SplineMeshList`)))
        (:`Is Not Valid`
          (bind _returnvalue (`AddComponent|NODE_AddSplineComponent-1`))
          (set `self.SplineComponent` _returnvalue)))
      (bind _returnvalue_2 (`|GetDataTableRow` "/Game/Blueprints/DB/DB_CommonMarker.DB_CommonMarker" "Location")
        (:`then`
          (bind _returnvalue_3 (`|SpawnActorFromClass` "/Game/Blueprints/Common/Map/BP_CommonMarker.BP_CommonMarker_C" (`KismetMathLibrary.Conv_VectorToTransform` (`local.FinalLocation`)) "Undefined" "OverrideRootScale" null "NewEnumerator2" _returnvalue_2 null))
          (set `self.RoutePin` _returnvalue_3)
          (bind _returnvalue_4 (`KismetSystemLibrary.K2_SetTimerDelegate` (`|CreateDelegate` :!event `DrawRoute`) 0.2 true))
          (set `self.DrawRouteTimer` _returnvalue_4))))))

(fn `UserConstructionScript`
  (bind (_returnvalue_x _returnvalue_y) (break `IntVector` (`GameplayStatics.GetWorldOriginLocation`)))
  (bind _returnvalue (`KismetMathLibrary.SafeDivide` (`self.WorldSizeInUnits`) 100.0))
  (`self.K2_SetActorLocation` (`KismetMathLibrary.MakeVector` (`KismetMathLibrary.Conv_IntToDouble` (/ _returnvalue_x 2)) (`KismetMathLibrary.Conv_IntToDouble` (/ _returnvalue_y 2))))
  (set `self.WorldSizeInUnits` (* (`self.WorldSizeInKm`) 100000.0))
  (`SceneComponent.K2_SetRelativeLocation` (`self.Camera`) (`KismetMathLibrary.MakeVector` 0.0 0.0 (`self.WorldSizeInUnits`)) false false)
  (`SceneComponent.SetRelativeScale3D` (`self.ProjectionPlane`) (`KismetMathLibrary.MakeVector` _returnvalue _returnvalue 1.0))
  (if (`self.bCapture`)
    (`self.MakeMapCapture`)))