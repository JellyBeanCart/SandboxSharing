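; Editor utility actor that bakes the material pattern on a plane into a noise texture PNG under the content Textures/Noise folder.
; The construction script creates a render target and fits an orthographic scene capture, showing only the plane, to the pattern scale.
; Preview flags drive the material's red, green and blue parameters.
; The Capture bool acts as a one-shot button, exporting and resetting only when all previews are off.
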(fn `UserConstructionScript`
  (bind _texturesize (`self.TextureSize`))
  (bind _returnvalue (`KismetMathLibrary.Conv_IntToDouble` (`self.PatternScale`)))
  (bind _returnvalue_2 (`KismetRenderingLibrary.CreateRenderTarget2D` _texturesize _texturesize))
  (bind _output_get (set `self.RT_Noise` _returnvalue_2))
  (set `SceneCaptureComponent2D.TextureTarget` _output_get (`self.SceneCaptureComponent2D`))
  (`SceneCaptureComponent.ShowOnlyComponent` (`self.SceneCaptureComponent2D`) (`self.Plane`))
  (`SceneComponent.SetRelativeScale3D` (`self.Plane`) (`KismetMathLibrary.MakeVector` _returnvalue _returnvalue 1.0))
  (set `SceneCaptureComponent2D.OrthoWidth` (* (`self.PatternScale`) 100.0) (`self.SceneCaptureComponent2D`))
  (`MeshComponent.SetScalarParameterValueOnMaterials` (`self.Plane`) "Red" (`KismetMathLibrary.SelectFloat` 1.0 0.0 (`self.bPreviewRedChannel`)))
  (`MeshComponent.SetScalarParameterValueOnMaterials` (`self.Plane`) "Green" (`KismetMathLibrary.SelectFloat` 1.0 0.0 (`self.bPreviewGreenChannel`)))
  (`MeshComponent.SetScalarParameterValueOnMaterials` (`self.Plane`) "Blue" (`KismetMathLibrary.SelectFloat` 1.0 0.0 (`self.bPreviewBlueChannel`)))
  (if (and (`self.bCapture`) (not (or (`self.bPreviewRedChannel`) (`self.bPreviewGreenChannel`) (`self.bPreviewBlueChannel`))))
    (`SceneCaptureComponent2D.CaptureScene` (`self.SceneCaptureComponent2D`))
    (`KismetRenderingLibrary.ExportRenderTarget` (`self.RT_Noise`) (`KismetStringLibrary.Concat_StrStr` (`KismetSystemLibrary.GetProjectContentDirectory`) "Textures/Noise") (`KismetMathLibrary.SelectString` (`KismetStringLibrary.Concat_StrStr` "T_" (`self.TextureName`) "_" (`KismetStringLibrary.Conv_IntToString` (`self.TextureSize`)) ".png") (`KismetStringLibrary.Concat_StrStr` "T_" "GeneratedNoise_" (`KismetStringLibrary.Conv_IntToString` (`self.TextureSize`)) ".png") (`KismetStringLibrary.NotEqual_StrStr` (`self.TextureName`))))
    (set `self.bCapture` false)))