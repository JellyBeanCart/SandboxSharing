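; BP_POI is a point-of-interest trigger that shows a typed-out text description and moves the camera to itself when the player enters its box.
; The overlap fires once, passing its text and letter delay to the player controller and blending the view target to the POI.
; DestroyDescriptionWidget blends the view back to the player character.
; The construction script sizes the trigger box from the CollisionBox variable.
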(event `self.Box.OnComponentBeginOverlap`
  (params (OverlappedComponent :type "PrimitiveComponent Object Reference") (OtherActor :type "Actor Object Reference") (OtherComp :type "PrimitiveComponent Object Reference") (OtherBodyIndex :type Integer) (bFromSweep :type Boolean) (SweepResult :type "HitResult Structure (by ref)"))
  (cast `/Game/Blueprints/Core/BP_PlayerCharacter` OtherActor)
  (`/Engine/EditorBlueprintResources/StandardMacros.DoOnce` false
    (:`Completed`
      (message `/Game/Blueprints/Interfaces/BPI_InteractionSystem.AddDescriptionWidget` (`GameplayStatics.GetPlayerController` 0) self null (`self.Text`) (`self.DelayBetweenLetters`))
      (`PlayerController.SetViewTargetWithBlend` (`GameplayStatics.GetPlayerController` 0) self (`self.BlendInTime`) "VTBlend_Linear" 0.0 false))))

(event `/Game/Blueprints/Interfaces/BPI_InteractionSystem.DestroyDescriptionWidget`
  (`PlayerController.SetViewTargetWithBlend` (`GameplayStatics.GetPlayerController` 0) (`GameplayStatics.GetPlayerCharacter` 0) (`self.BlendOutTime`) "VTBlend_Linear" 0.0 false))

(fn `GetActiveConsumableWidget`
  (returns (GUI_Consumable :type "/Game/GUI/HUD/HUD_Consumable Object Reference"))
  (return null))

(fn `GetPieMenuWidget`
  (returns (GUI_PieMenu :type "/Game/GUI/HUD/HUD_PieMenu Object Reference"))
  (return null))

(fn `UserConstructionScript`
  (`BoxComponent.SetBoxExtent` (`self.Box`) (/ (`self.CollisionBox`) 2.0) true))