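; Quest component that runs a sequence of DataTable-defined quests and tracks the player's progress through them.
; It restores saved progress on a matching checkpoint level, otherwise selecting the first quest.
; Quest updates match Reach, Iterate/Consume and Interact/Grab/Release steps by type and object, update the quest widget, then advance quests or flag the next chapter.
; A looping timer waits for the widget, and GetCurrentQuest packages progression state.
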(event `/Game/Blueprints/Interfaces/BPI_QuestSystem.SetQuestDB`
  (params (QuestDB :type "DataTable Object Reference"))
  (bind _output_get (set `self.QuestDB` QuestDB))
  (bind _outrownames (`DataTableFunctionLibrary.GetDataTableRowNames` _output_get))
  (bind _output_get_2 (set `self.QuestNames` _outrownames))
  (for _array_element _output_get_2
    (bind _returnvalue (`|GetDataTableRow` (`self.QuestDB`) _array_element)
      (:`then`
        (`KismetArrayLibrary.Array_AddUnique` (`self.QuestDataList`) _returnvalue))))
  (bind _gamedata (message `/Game/Blueprints/Interfaces/BPI_GameInstance.LoadGameData` (`GameplayStatics.GetGameInstance`)))
  (set `self.GameData` _gamedata)
  (set `self.CompletedStepsAmount` (`.CompletedSteps_7_6BEE4466473465D2F0A4779838688168` (break `/Game/Blueprints/Structures/QuestChildren/FQuestProgression` (`.Progression_41_19F67DB4460BA060ECAC96ACA2AC3E50` (break `/Game/Blueprints/Structures/GameDataChildren/FPlayerData` (`.Player_34_DD80CB954E9A40AF1BD1338114B3921E` (break `/Game/Blueprints/Structures/FGameData` (`self.GameData`))))))))
  (set `self.CurrentQuestIndex` (`.CurrentQuestIndex_5_A1D4BD474B1641FE217C11BEF567306F` (break `/Game/Blueprints/Structures/QuestChildren/FQuestProgression` (`.Progression_41_19F67DB4460BA060ECAC96ACA2AC3E50` (break `/Game/Blueprints/Structures/GameDataChildren/FPlayerData` (`.Player_34_DD80CB954E9A40AF1BD1338114B3921E` (break `/Game/Blueprints/Structures/FGameData` (`self.GameData`))))))))
  (set `self.CurrentQuestData` (`.CurrentQuestData_2_F1375AEF43C93C6009B188AFFCD4AA61` (break `/Game/Blueprints/Structures/QuestChildren/FQuestProgression` (`.Progression_41_19F67DB4460BA060ECAC96ACA2AC3E50` (break `/Game/Blueprints/Structures/GameDataChildren/FPlayerData` (`.Player_34_DD80CB954E9A40AF1BD1338114B3921E` (break `/Game/Blueprints/Structures/FGameData` (`self.GameData`))))))))
  (set `self.bGoNextChapter` (`.bGoNextChapter_10_92DCC49E439B92CEEA81B5A88A5EA64D` (break `/Game/Blueprints/Structures/QuestChildren/FQuestProgression` (`.Progression_41_19F67DB4460BA060ECAC96ACA2AC3E50` (break `/Game/Blueprints/Structures/GameDataChildren/FPlayerData` (`.Player_34_DD80CB954E9A40AF1BD1338114B3921E` (break `/Game/Blueprints/Structures/FGameData` (`self.GameData`))))))))
  (bind _returnvalue_2 (`GameplayStatics.GetCurrentLevelName` true))
  (if (`KismetStringLibrary.EqualEqual_StrStr` _returnvalue_2 (`.Checkpoint_30_178B22014272EB4EEB4CBF8480A61A3B` (break `/Game/Blueprints/Structures/GameDataChildren/FLevelData` (`.Level_37_C2FF1CFD417204E825B165B1F75E41BE` (break `/Game/Blueprints/Structures/FGameData` (`self.GameData`))))))
    (if (not (`KismetStringLibrary.NotEqual_StrStr` (`.Description_4_1C0034DF4F1CA97466E423B356F25962` (break `/Game/Blueprints/Structures/FQuest` (`self.CurrentQuestData`)))))
      (bind _output_get_3 (set `self.CurrentQuestIndex` 0 :!label _label))
      (set `self.CurrentQuestData` (`|GetArrayItem` (`self.QuestDataList`) _output_get_3)))
    (else
      (goto _label)))
  (add `self.OnQuestItemIterated` (`|CreateDelegate` :!event `UpdateQuest`))
  (add `self.OnCheckpointReached` (`|CreateDelegate` :!event `UpdateQuest`))
  (add `self.OnQuestItemInteracted` (`|CreateDelegate` :!event `UpdateQuest`)))

(event `ValidateQuestWidget`
  (bind _gui_quest (message `/Game/Blueprints/Interfaces/BPI_QuestSystem.GetQuestWidget` (`GameplayStatics.GetPlayerController` 0)))
  (`/Engine/EditorBlueprintResources/StandardMacros.IsValid` _gui_quest
    (:`Is Valid`
      (set `self.GUI_Quest` _gui_quest)
      (`KismetSystemLibrary.K2_ClearAndInvalidateTimerHandle` (`self.ValidateQuestWidgetTimer`))
      (`/Game/GUI/HUD/HUD_Quest.StartQuest` (`self.GUI_Quest`) (`self.CurrentQuestData`)))))

(event `/Game/Blueprints/Interfaces/BPI_QuestSystem.StartQuest`
  (bind (_reach _iterate _interact) (break `/Game/Blueprints/Structures/QuestChildren/FQuestSteps` (`.Steps_13_B4D8E0F74C1FA9002CCC74BA78922CE4` (break `/Game/Blueprints/Structures/FQuest` (`self.CurrentQuestData`)))))
  (set `self.InitialStepsAmount` (+ (`KismetArrayLibrary.Array_Length` _reach) (`KismetArrayLibrary.Array_Length` _iterate) (`KismetArrayLibrary.Array_Length` _interact)) :!label _label_2)
  (`/Engine/EditorBlueprintResources/StandardMacros.IsValid` (`self.GUI_Quest`)
    (:`Is Valid`
      (`/Game/GUI/HUD/HUD_Quest.StartQuest` (`self.GUI_Quest`) (`self.CurrentQuestData`)))
    (:`Is Not Valid`
      (bind _returnvalue (`KismetSystemLibrary.K2_SetTimerDelegate` (`|CreateDelegate` :!event `ValidateQuestWidget`) 0.2 true))
      (set `self.ValidateQuestWidgetTimer` _returnvalue))))

(event `NextQuest`
  (set `self.CurrentQuestData` (`|GetArrayItem` (`self.QuestDataList`) (`self.CurrentQuestIndex`)))
  (goto _label_2))

(event `/Game/Blueprints/Interfaces/BPI_QuestSystem.CompleteQuest`
  (`/Game/GUI/HUD/HUD_Quest.CompleteQuest` (`self.GUI_Quest`))
  (set `self.CompletedStepsAmount` 0)
  (set `self.CurrentQuestIndex` (+ (`self.CurrentQuestIndex`) 1))
  (if (not (> (`self.CurrentQuestIndex`) (`KismetArrayLibrary.Array_LastIndex` (`self.QuestDataList`))))
    (`KismetSystemLibrary.K2_SetTimerDelegate` (`|CreateDelegate` :!event `NextQuest`) 0.02)
    (else
      (set `self.bGoNextChapter` true))))

(event `/Game/Blueprints/Interfaces/BPI_QuestSystem.UpdateQuest`
  (params (Type :type "/Game/Blueprints/Enumerations/EQuestType Enum" :default "NewEnumerator0") (Object :type "/Game/Blueprints/Common/InteractionSystem/BP_InteractableBase Class Reference"))
  (`self.ComputeQuestSteps` Type Object)
  (if (>= (`self.CompletedStepsAmount`) (`self.InitialStepsAmount`))
    (`/Game/Blueprints/Interfaces/BPI_QuestSystem.CompleteQuest`)))

(fn `ComputeQuestSteps`
  (params (Type :type "/Game/Blueprints/Enumerations/EQuestType Enum" :default "NewEnumerator0") (Object :type "/Game/Blueprints/Common/InteractionSystem/BP_InteractableBase Class Reference"))
  (locals (IterationAmount :type Integer) (IterationIndex :type Integer) (ReachIndex :type Integer) (InteractIndex :type Integer))
  (switch `/Game/Blueprints/Enumerations/EQuestType` (`local.Type`)
    (:`NewEnumerator1`
      (for (_array_element _array_index) (`.Iterate_9_C8DEBE284B3097DE59132D9EF5DD30D6` (break `/Game/Blueprints/Structures/QuestChildren/FQuestSteps` (`.Steps_13_B4D8E0F74C1FA9002CCC74BA78922CE4` (break `/Game/Blueprints/Structures/FQuest` (`self.CurrentQuestData`))))) :!label _label
        (set `local.IterationIndex` _array_index)
        (bind ((`Object_5_118B76D64A2E019A1D50B19494A9771B` _object) (`bCompleted_13_363F890A45FBD33E11D09A90DC25AC4D` _bcompleted) (`Type_16_1CADF3904BB37BDCB98D3ABF44A58AE5` _type) (`CurrentAmount_20_0A9E0E624F7F420AD2298F9212F43E83` _currentamount) (`MaxAmount_17_4B6F45A14B6B6D766E3C23AFE000DF40` _maxamount)) (break `/Game/Blueprints/Structures/QuestChildren/FQuestIterate` _array_element))
        (if (and (== _object (`local.Object`)) (not _bcompleted) (`|EnumEquality` _type (`local.Type`)))
          (bind _output_get (set `local.IterationAmount` (+ _currentamount 1)))
          (setmembers `/Game/Blueprints/Structures/QuestChildren/FQuestIterate` :`StructRef` (`|GetArrayItem` (`.Iterate_9_C8DEBE284B3097DE59132D9EF5DD30D6` (break `/Game/Blueprints/Structures/QuestChildren/FQuestSteps` (`.Steps_13_B4D8E0F74C1FA9002CCC74BA78922CE4` (break `/Game/Blueprints/Structures/FQuest` (`self.CurrentQuestData`))))) (`local.IterationIndex`)) :`CurrentAmount` _output_get)
          (if (>= (`local.IterationAmount`) _maxamount)
            (bind _structout (setmembers `/Game/Blueprints/Structures/QuestChildren/FQuestIterate` :`StructRef` (`|GetArrayItem` (`.Iterate_9_C8DEBE284B3097DE59132D9EF5DD30D6` (break `/Game/Blueprints/Structures/QuestChildren/FQuestSteps` (`.Steps_13_B4D8E0F74C1FA9002CCC74BA78922CE4` (break `/Game/Blueprints/Structures/FQuest` (`self.CurrentQuestData`))))) (`local.IterationIndex`)) :`bCompleted` true))
            (set `self.CompletedStepsAmount` (+ (`self.CompletedStepsAmount`) 1)))
          (`/Game/GUI/HUD/HUD_Quest.UpdateStep` (`self.GUI_Quest`) (`.Description_2_122DB17D4F65EC639B03F2A01B4FCB98` (break `/Game/Blueprints/Structures/QuestChildren/FQuestIterate` _structout))))))
    (:`NewEnumerator2`
      (for (_array_element_2 _array_index_2) (`.Reach_10_0381C42F4501D141D271EE898F74F5B9` (break `/Game/Blueprints/Structures/QuestChildren/FQuestSteps` (`.Steps_13_B4D8E0F74C1FA9002CCC74BA78922CE4` (break `/Game/Blueprints/Structures/FQuest` (`self.CurrentQuestData`)))))
        (set `local.ReachIndex` _array_index_2)
        (bind ((`Checkpoint_20_118B76D64A2E019A1D50B19494A9771B` _checkpoint) (`bCompleted_16_7D01E1474805EF1DAEAC70B1E276F64E` _bcompleted_2) (`Type_23_EB1FD7F148B03808CEF3748358D268C8` _type_2)) (break `/Game/Blueprints/Structures/QuestChildren/FQuestReach` _array_element_2))
        (if (and (== _checkpoint (`local.Object`)) (not _bcompleted_2) (`|EnumEquality` _type_2 (`local.Type`)))
          (bind _structout_2 (setmembers `/Game/Blueprints/Structures/QuestChildren/FQuestReach` :`StructRef` (`|GetArrayItem` (`.Reach_10_0381C42F4501D141D271EE898F74F5B9` (break `/Game/Blueprints/Structures/QuestChildren/FQuestSteps` (`.Steps_13_B4D8E0F74C1FA9002CCC74BA78922CE4` (break `/Game/Blueprints/Structures/FQuest` (`self.CurrentQuestData`))))) (`local.ReachIndex`)) :`bCompleted` true))
          (`/Game/GUI/HUD/HUD_Quest.UpdateStep` (`self.GUI_Quest`) (`.Description_2_122DB17D4F65EC639B03F2A01B4FCB98` (break `/Game/Blueprints/Structures/QuestChildren/FQuestReach` _structout_2)))
          (set `self.CompletedStepsAmount` (+ (`self.CompletedStepsAmount`) 1)))))
    (:`NewEnumerator3`
      (for (_array_element_3 _array_index_3) (`.Interact_11_CE024D514BBD62FF9291C9B1F3B55313` (break `/Game/Blueprints/Structures/QuestChildren/FQuestSteps` (`.Steps_13_B4D8E0F74C1FA9002CCC74BA78922CE4` (break `/Game/Blueprints/Structures/FQuest` (`self.CurrentQuestData`))))) :!label _label_2
        (set `local.InteractIndex` _array_index_3)
        (bind ((`Object_17_A25CA9E3406EE9282A83ABB403601B72` _object_2) (`bCompleted_19_75DAE98649272983F8AD6CBC28A13D61` _bcompleted_3) (`Type_22_4605D7284B28C1741279AD972FE97B9E` _type_3)) (break `/Game/Blueprints/Structures/QuestChildren/FQuestInteract` _array_element_3))
        (if (and (== _object_2 (`local.Object`)) (not _bcompleted_3) (`|EnumEquality` _type_3 (`local.Type`)))
          (bind _structout_3 (setmembers `/Game/Blueprints/Structures/QuestChildren/FQuestInteract` :`StructRef` (`|GetArrayItem` (`.Interact_11_CE024D514BBD62FF9291C9B1F3B55313` (break `/Game/Blueprints/Structures/QuestChildren/FQuestSteps` (`.Steps_13_B4D8E0F74C1FA9002CCC74BA78922CE4` (break `/Game/Blueprints/Structures/FQuest` (`self.CurrentQuestData`))))) (`local.InteractIndex`)) :`bCompleted` true))
          (`/Game/GUI/HUD/HUD_Quest.UpdateStep` (`self.GUI_Quest`) (`.Description_2_122DB17D4F65EC639B03F2A01B4FCB98` (break `/Game/Blueprints/Structures/QuestChildren/FQuestInteract` _structout_3)))
          (set `self.CompletedStepsAmount` (+ (`self.CompletedStepsAmount`) 1)))))
    (:`NewEnumerator4`
      (goto _label))
    (:`NewEnumerator5`
      (goto _label_2))
    (:`NewEnumerator6`
      (goto _label_2))))

(fn `GetCurrentQuest`
  (returns (QuestProgression :type "/Game/Blueprints/Structures/QuestChildren/FQuestProgression Structure"))
  (return (make `/Game/Blueprints/Structures/QuestChildren/FQuestProgression` (`self.CompletedStepsAmount`) (`self.CurrentQuestIndex`) (`self.CurrentQuestData`) (`self.bGoNextChapter`))))

(fn `GetQuestWidget`
  (returns (GUI_Quest :type "/Game/GUI/HUD/HUD_Quest Object Reference"))
  (return null))