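; Day/night and weather controller that advances a 24-hour clock from the configured day length, starting from the level's saved time when one exists.
; Curves sampled by that time rotate sun and moon and set light intensities, sky and fog, volumetric cloud material, and rain, snow, lightning and star effects.
; Effect components attach to the player once it is valid, and rain and snow amounts feed MPC_Weather.
; The construction script applies the same update.
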(event `CheckPlayerReady`
  (`/Engine/EditorBlueprintResources/StandardMacros.IsValid` (`/Game/Blueprints/FunctionLibrary/BP_FunctionLibrary.GetPlayerCharacter`)
    (:`Is Valid`
      (`KismetSystemLibrary.K2_ClearAndInvalidateTimerHandle` (`self.CheckPlayerTimer`))
      (`SceneComponent.K2_AttachToComponent` (`self.RainComponent`) (`Actor.RootComponent` (`/Game/Blueprints/FunctionLibrary/BP_FunctionLibrary.GetPlayerCharacter`)) "None" "SnapToTarget" "KeepRelative" "KeepRelative" true)
      (`SceneComponent.K2_AttachToComponent` (`self.SnowComponent`) (`Actor.RootComponent` (`/Game/Blueprints/FunctionLibrary/BP_FunctionLibrary.GetPlayerCharacter`)) "None" "SnapToTarget" "KeepRelative" "KeepRelative" true)
      (`SceneComponent.K2_AttachToComponent` (`self.StarsComponent`) (`Actor.RootComponent` (`/Game/Blueprints/FunctionLibrary/BP_FunctionLibrary.GetPlayerCharacter`)) "None" "SnapToTarget" "KeepRelative" "KeepRelative" true)
      (`SceneComponent.K2_AttachToComponent` (`self.LightningComponent`) (`Actor.RootComponent` (`/Game/Blueprints/FunctionLibrary/BP_FunctionLibrary.GetPlayerCharacter`)) "None" "SnapToTarget" "KeepRelative" "KeepRelative" true))))

(event `self.ReceiveBeginPlay`
  (bind (_value _returnvalue) (`BlueprintMapLibrary.Map_Find` (`.LevelsTime_36_B3FEAA4A4A957489993C0C9C92713D23` (break `/Game/Blueprints/Structures/GameDataChildren/FLevelData` (`self.LevelData`))) (`self.CurrentLevel`)))
  (set `self.OneHour` (/ (* (`self.DayLengthInMinutes`) 60.0) 24.0))
  (bind _returnvalue_2 (`KismetSystemLibrary.K2_SetTimerDelegate` (`|CreateDelegate` :!event `CheckPlayerReady`) 0.2 true))
  (set `self.CheckPlayerTimer` _returnvalue_2)
  (bind _returnvalue_3 (`GameplayStatics.GetCurrentLevelName` true))
  (set `self.CurrentLevel` _returnvalue_3)
  (bind _gamedata (message `/Game/Blueprints/Interfaces/BPI_GameInstance.LoadGameData` (`GameplayStatics.GetGameInstance`)))
  (set `self.LevelData` (`.Level_37_C2FF1CFD417204E825B165B1F75E41BE` (break `/Game/Blueprints/Structures/FGameData` _gamedata)))
  (if _returnvalue
    (set `self.CurrentTime` _value)
    (else
      (set `self.CurrentTime` (`self.CurrentTime`)))))

(event `self.ReceiveTick`
  (params (DeltaSeconds :type "Float (single-precision)"))
  (bind _returnvalue (+ (`KismetMathLibrary.SafeDivide` DeltaSeconds (`self.OneHour`)) (`self.CurrentTime`)))
  (if (> _returnvalue 0.0)
    (if (<= _returnvalue 24.0)
      (set `self.CurrentTime` _returnvalue)
      (else
        (set `self.CurrentTime` (`KismetMathLibrary.Abs` (- 24.0 _returnvalue)))))
    (`self.K2_SetActorRotation` (`self.Sun`) (`KismetMathLibrary.MakeRotator` 0.0 (`CurveFloat.GetFloatValue` (`self.DayLengthCurve`) (`self.CurrentTime`))) false)
    (`self.K2_SetActorRotation` (`self.Moon`) (`KismetMathLibrary.MakeRotator` 0.0 (* (`CurveFloat.GetFloatValue` (`self.DayLengthCurve`) (`self.CurrentTime`)) -1.0)) false)
    (`self.UpdateWeather`)
    (`self.UpdateWorldFeedback`)))

(fn `UpdateWeather`
  (locals (WeatherType :type "Float (double-precision)" :default 0.0))
  (bind _currenttime (`self.CurrentTime`))
  (bind (_returnvalue_x _returnvalue_y) (`KismetMathLibrary.BreakVector` (`CurveVector.GetVectorValue` (`self.SunIntensityCurve`) (`self.CurrentTime`))))
  (bind (_returnvalue_x_2 _returnvalue_y_2) (`KismetMathLibrary.BreakVector` (`CurveVector.GetVectorValue` (`self.SkyLightIntensityCurve`) (`self.CurrentTime`))))
  (bind (_returnvalue_x_3 _returnvalue_y_3) (`KismetMathLibrary.BreakVector` (`CurveVector.GetVectorValue` (`self.CloudOpacityCurve`) (`self.CurrentTime`))))
  (bind _returnvalue_x_4 (`KismetMathLibrary.BreakVector` (`CurveVector.GetVectorValue` (`self.CloudOpacityCurve`) (`self.CurrentTime`))))
  (bind _returnvalue_x_5 (`KismetMathLibrary.BreakVector` (`CurveVector.GetVectorValue` (`self.SnowCurve`) (`self.CurrentTime`))))
  (bind (_returnvalue_x_6 _returnvalue_y_4) (`KismetMathLibrary.BreakVector` (`CurveVector.GetVectorValue` (`self.CloudOpacityCurve`) (`self.CurrentTime`))))
  (bind (_returnvalue_x_7 _returnvalue_y_5) (`KismetMathLibrary.BreakVector` (`CurveVector.GetVectorValue` (`self.MoonIntensityCurve`) (`self.CurrentTime`))))
  (bind (_returnvalue_x_8 _returnvalue_y_6) (`KismetMathLibrary.BreakVector` (/ (`self.StardomRotationSpeed`) (`self.DayLengthInMinutes`))))
  (bind _returnvalue (`self.GetComponentByClass` (`self.Sun`) "/Script/Engine.DirectionalLightComponent"))
  (bind _returnvalue_2 (`self.GetComponentByClass` (`self.Sun`) "/Script/Engine.DirectionalLightComponent"))
  (bind _returnvalue_x_9 (`KismetMathLibrary.BreakVector` (`CurveVector.GetVectorValue` (`self.RainCurve`) (`self.CurrentTime`))))
  (set `local.WeatherType` (`CurveFloat.GetFloatValue` (`self.WeatherTypeCurve`) (`self.CurrentTime`)))
  (`LightComponent.SetIntensity` (`Light.LightComponent` (`self.Sun`)) (`KismetMathLibrary.Lerp` _returnvalue_x _returnvalue_y (`local.WeatherType`)))
  (`LightComponent.SetIntensity` (`Light.LightComponent` (`self.Moon`)) (`KismetMathLibrary.Lerp` _returnvalue_x_7 _returnvalue_y_5 (`local.WeatherType`)))
  (`SkyLightComponent.SetIntensity` (`SkyLight.LightComponent` (`self.SkyLight`)) (`KismetMathLibrary.Lerp` _returnvalue_x_2 _returnvalue_y_2 (`local.WeatherType`)))
  (if (> _returnvalue_y_3 0.5)
    (`ActorComponent.Activate` (`self.LightningComponent`) false)
    (else
      (`ActorComponent.Deactivate` (`self.LightningComponent`))))
  (if (`self.bRain`)
    (if (`KismetMathLibrary.NearlyEqual_FloatFloat` _returnvalue_x_9 1.0)
      (`ActorComponent.Activate` (`self.RainComponent`) false)
      (set `self.bIsRaining` true)
      (else
        (`ActorComponent.Deactivate` (`self.RainComponent`))
        (set `self.bIsRaining` false)))
    (else
      (`ActorComponent.Deactivate` (`self.RainComponent`))
      (set `self.bIsRaining` false)))
  (if (`self.bSnow`)
    (if (`KismetMathLibrary.NearlyEqual_FloatFloat` _returnvalue_x_5 1.0)
      (`ActorComponent.Activate` (`self.SnowComponent`) false)
      (set `self.bIsSnowing` true)
      (else
        (`ActorComponent.Deactivate` (`self.SnowComponent`))
        (set `self.bIsSnowing` false)))
    (else
      (`ActorComponent.Deactivate` (`self.SnowComponent`))
      (set `self.bIsSnowing` false)))
  (if (`self.bFog`)
    (`ExponentialHeightFogComponent.SetFogDensity` (`ExponentialHeightFog.Component` (`self.Fog`)) (`CurveFloat.GetFloatValue` (`self.FogDensityCurve`) (`self.CurrentTime`)))
    (else
      (`ExponentialHeightFogComponent.SetFogDensity` (`ExponentialHeightFog.Component` (`self.Fog`)) 0.005)))
  (if (and (> _currenttime 6.0) (< _currenttime 18.0))
    (`DirectionalLightComponent.SetEnableLightShaftOcclusion` _returnvalue_2 true)
    (`LightComponent.SetEnableLightShaftBloom` _returnvalue_2 true)
    (else
      (`DirectionalLightComponent.SetEnableLightShaftOcclusion` _returnvalue false)
      (`LightComponent.SetEnableLightShaftBloom` _returnvalue false)))
  (`SkyAtmosphereComponent.SetRayleighScattering` (`SkyAtmosphere.SkyAtmosphereComponent` (`self.SkyAtmosphere`)) (`KismetMathLibrary.LinearColorLerp` (`self.SunnySkyColor`) (`self.CloudySkyColor`) (`local.WeatherType`)))
  (`ExponentialHeightFogComponent.SetFogInscatteringColor` (`ExponentialHeightFog.Component` (`self.Fog`)) (`KismetMathLibrary.LinearColorLerp` (`CurveLinearColor.GetClampedLinearColorValue` (`self.FogSunnyColorCurve`) (`KismetMathLibrary.NormalizeToRange` (`self.CurrentTime`) 0.0 24.0)) (`CurveLinearColor.GetClampedLinearColorValue` (`self.FogCloudyColorCurve`) (`KismetMathLibrary.NormalizeToRange` (`self.CurrentTime`) 0.0 24.0)) (`CurveFloat.GetFloatValue` (`self.WeatherTypeCurve`) (`self.CurrentTime`))))
  (`MaterialInstanceDynamic.SetScalarParameterValue` (`self.MID_VolumetricClouds`) "StratusCoverage" _returnvalue_x_4)
  (`MaterialInstanceDynamic.SetScalarParameterValue` (`self.MID_VolumetricClouds`) "CumulonimbusCoverage" _returnvalue_y_4)
  (`MaterialInstanceDynamic.SetScalarParameterValue` (`self.MID_VolumetricClouds`) "CloudSpeedX" (`KismetMathLibrary.SafeDivide` (`self.CloudSpeedX`) (`self.DayLengthInMinutes`)))
  (`MaterialInstanceDynamic.SetScalarParameterValue` (`self.MID_VolumetricClouds`) "CloudSpeedY" (`KismetMathLibrary.SafeDivide` (`self.CloudSpeedY`) (`self.DayLengthInMinutes`)))
  (if (`KismetMathLibrary.NearlyEqual_FloatFloat` (`CurveFloat.GetFloatValue` (`self.StarsCurve`) (`self.CurrentTime`)) 1.0)
    (`ActorComponent.Activate` (`self.StarsComponent`) false)
    (`NiagaraComponent.SetVariableVec3` (`self.StarsComponent`) "StardomRotation" (`KismetMathLibrary.MakeVector` _returnvalue_x_8 _returnvalue_y_6))
    (else
      (`ActorComponent.Deactivate` (`self.StarsComponent`)))))

(fn `UpdateWorldFeedback`
  (bind (_returnvalue_x _returnvalue_y) (`KismetMathLibrary.BreakVector` (`CurveVector.GetVectorValue` (`self.RainCurve`) (`self.CurrentTime`))))
  (bind (_returnvalue_x_2 _returnvalue_y_2) (`KismetMathLibrary.BreakVector` (`CurveVector.GetVectorValue` (`self.SnowCurve`) (`self.CurrentTime`))))
  (`KismetMaterialLibrary.SetVectorParameterValue` "/Game/Materials/MPC/MPC_Weather.MPC_Weather" "Conditions" (`KismetMathLibrary.MakeColor` _returnvalue_y _returnvalue_y_2)) ; Rain
  (`KismetMaterialLibrary.SetVectorParameterValue` "/Game/Materials/MPC/MPC_Weather.MPC_Weather" "Conditions" (`KismetMathLibrary.MakeColor` _returnvalue_y _returnvalue_y_2)) ; Snow
)

(fn `UserConstructionScript`
  (`self.K2_SetActorLocation` (`KismetMathLibrary.Conv_IntVectorToVector` (`GameplayStatics.GetWorldOriginLocation`)))
  (`/Engine/EditorBlueprintResources/StandardMacros.IsValid` (`self.Sun`)
    (:`Is Valid`
      (`/Engine/EditorBlueprintResources/StandardMacros.IsValid` (`self.Moon`)
        (:`Is Valid`
          (`/Engine/EditorBlueprintResources/StandardMacros.IsValid` (`self.SkyLight`)
            (:`Is Valid`
              (`/Engine/EditorBlueprintResources/StandardMacros.IsValid` (`self.SkyAtmosphere`)
                (:`Is Valid`
                  (`/Engine/EditorBlueprintResources/StandardMacros.IsValid` (`self.VolumetricClouds`)
                    (:`Is Valid`
                      (`/Engine/EditorBlueprintResources/StandardMacros.IsValid` (`self.Fog`)
                        (:`Is Valid`
                          (`self.K2_SetActorRotation` (`self.Sun`) (`KismetMathLibrary.MakeRotator` 0.0 (`CurveFloat.GetFloatValue` (`self.DayLengthCurve`) (`self.CurrentTime`))) false)
                          (`self.K2_SetActorRotation` (`self.Moon`) (`KismetMathLibrary.MakeRotator` 0.0 (* (`CurveFloat.GetFloatValue` (`self.DayLengthCurve`) (`self.CurrentTime`)) -1.0)) false)
                          (bind _returnvalue (`KismetMaterialLibrary.CreateDynamicMaterialInstance` "/Game/Materials/VolumetricClouds/MI_VolumetricClouds.MI_VolumetricClouds"))
                          (bind _output_get (set `self.MID_VolumetricClouds` _returnvalue))
                          (`VolumetricCloudComponent.SetMaterial` (`VolumetricCloud.VolumetricCloudComponent` (`self.VolumetricClouds`)) _output_get)
                          (`self.UpdateWeather`)
                          (`self.UpdateWorldFeedback`))))))))))))))