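; BP_GameMenuController is a player controller that owns and displays the main menu.
; On BeginPlay it creates the GUI_MainMenu widget with a fixed GameMode enum value and adds it to the viewport at a high Z-order.
; Showing the menu switches input to UI-only with focus on the widget and enables the mouse cursor.
; When the controller is destroyed, it removes the widget and clears the reference.
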(event `self.ReceiveBeginPlay`
  (`/Game/Blueprints/Interfaces/BPI_MainMenu.CreateMainMenu`)
  (`/Game/Blueprints/Interfaces/BPI_MainMenu.ShowMainMenu`))

(event `self.ReceiveDestroyed`
  (`/Game/Blueprints/Interfaces/BPI_MainMenu.DestroyMainMenu`))

(event `/Game/Blueprints/Interfaces/BPI_MainMenu.CreateMainMenu`
  (bind _returnvalue (`|CreateWidget` "/Game/GUI/UI/GUI_MainMenu.GUI_MainMenu_C" null "NewEnumerator2"))
  (set `self.GUI_MainMenu` _returnvalue))

(event `/Game/Blueprints/Interfaces/BPI_MainMenu.DestroyMainMenu`
  (`/Engine/EditorBlueprintResources/StandardMacros.IsValid` (`self.GUI_MainMenu`)
    (:`Is Valid`
      (`Widget.RemoveFromParent` (`self.GUI_MainMenu`))
      (set `self.GUI_MainMenu` null))))

(event `/Game/Blueprints/Interfaces/BPI_MainMenu.ShowMainMenu`
  (`UserWidget.AddToViewport` (`self.GUI_MainMenu`) 10000)
  (`WidgetBlueprintLibrary.SetInputMode_UIOnlyEx` self (`self.GUI_MainMenu`))
  (set `self.bShowMouseCursor` true))

(fn `UserConstructionScript`)