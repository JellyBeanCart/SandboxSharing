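; Player controller that owns the player's UI, from main menu and HUD widgets to map, inventory, pie menu and binoculars.
; BeginPlay prebuilds the main menu and applies settings loaded from the game instance.
; Events create, update, show or remove each widget; menu, map, inventory and pie menu also switch input modes, and the main menu pauses the game.
; Threat indicators are capped at three; several data getters return only defaults.
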(event `self.ReceiveBeginPlay`
  (`/Game/Blueprints/Interfaces/BPI_MainMenu.CreateMainMenu`)
  (`WidgetBlueprintLibrary.SetInputMode_GameOnly` self)
  (set `self.bShowMouseCursor` false)
  (bind _settings (message `/Game/Blueprints/Interfaces/BPI_GameInstance.LoadGameSettings` (`GameplayStatics.GetGameInstance`)))
  (`/Game/Blueprints/FunctionLibrary/BP_FunctionLibrary.ApplyGameSettings` _settings))

(event `self.ReceiveDestroyed`
  (`/Game/Blueprints/Interfaces/BPI_MainMenu.DestroyMainMenu`))

(event `/Game/Blueprints/Interfaces/BPI_MainMenu.CreateMainMenu`
  (bind _returnvalue (`|CreateWidget` "/Game/GUI/UI/GUI_MainMenu.GUI_MainMenu_C" null "NewEnumerator1"))
  (set `self.GUI_MainMenu` _returnvalue))

(event `/Game/Blueprints/Interfaces/BPI_MainMenu.DestroyMainMenu`
  (`/Engine/EditorBlueprintResources/StandardMacros.IsValid` (`self.GUI_MainMenu`)
    (:`Is Valid`
      (`Widget.RemoveFromParent` (`self.GUI_MainMenu`))
      (set `self.GUI_MainMenu` null))))

(event `/Game/Blueprints/Interfaces/BPI_MainMenu.ShowMainMenu`
  (`UserWidget.AddToViewport` (`self.GUI_MainMenu`) 10000)
  (`WidgetBlueprintLibrary.SetInputMode_UIOnlyEx` self (`self.GUI_MainMenu`))
  (bind _output_get (set `self.bShowMouseCursor` true))
  (`GameplayStatics.SetGamePaused` _output_get))

(event `/Game/Blueprints/Interfaces/BPI_MainMenu.HideMainMenu`
  (`/Engine/EditorBlueprintResources/StandardMacros.IsValid` (`self.GUI_MainMenu`)
    (:`Is Valid`
      (`Widget.RemoveFromParent` (`self.GUI_MainMenu`))
      (`WidgetBlueprintLibrary.SetInputMode_GameOnly` self)
      (bind _output_get (set `self.bShowMouseCursor` false))
      (`GameplayStatics.SetGamePaused` _output_get))))

(event `InputAction|Menu`
  (params (Key :type "Key Structure"))
  (:`Pressed`
    (`/Game/Blueprints/Interfaces/BPI_MainMenu.ShowMainMenu`)))

(event `/Game/Blueprints/Interfaces/BPI_InteractionSystem.UpdateLogWidget`
  (params (Consumable :type "/Game/Blueprints/Common/InteractionSystem/BP_ConsumableBase Object Reference") (LogID :type "/Game/Blueprints/Enumerations/ELogMessage Enum" :default "NewEnumerator0"))
  (`/Engine/EditorBlueprintResources/StandardMacros.IsValid` (`self.GUI_Log`)
    (:`Is Valid`
      (`/Game/GUI/HUD/HUD_Log.CreateLogText` (`self.GUI_Log`) Consumable LogID))))

(event `/Game/Blueprints/Interfaces/BPI_InteractionSystem.CreateLogWidget`
  (bind _returnvalue (`|CreateWidget` "/Game/GUI/HUD/HUD_Log.HUD_Log_C"))
  (bind _output_get (set `self.GUI_Log` _returnvalue))
  (`UserWidget.AddToViewport` _output_get 0))

(event `/Game/Blueprints/Interfaces/BPI_InteractionSystem.DestroyLogWidget`
  (`/Engine/EditorBlueprintResources/StandardMacros.IsValid` (`self.GUI_Log`)
    (:`Is Valid`
      (`Widget.RemoveFromParent` (`self.GUI_Log`))
      (set `self.GUI_Log` null))))

(event `/Game/Blueprints/Interfaces/BPI_PlayerCharacter.CreateAttributesWidget`
  (bind _returnvalue (`|CreateWidget` "/Game/GUI/HUD/HUD_PlayerAttributes.HUD_PlayerAttributes_C"))
  (bind _output_get (set `self.GUI_PlayerAttributes` _returnvalue))
  (`UserWidget.AddToViewport` _output_get 0))

(event `/Game/Blueprints/Interfaces/BPI_PlayerCharacter.DestroyAttributesWidget`
  (`/Engine/EditorBlueprintResources/StandardMacros.IsValid` (`self.GUI_PlayerAttributes`)
    (:`Is Valid`
      (`Widget.RemoveFromParent` (`self.GUI_PlayerAttributes`))
      (set `self.GUI_PlayerAttributes` null))))

(event `/Game/Blueprints/Interfaces/BPI_InteractionSystem.CreatePointer`
  (bind _returnvalue (`|CreateWidget` "/Game/GUI/HUD/HUD_Pointer.HUD_Pointer_C"))
  (bind _output_get (set `self.GUI_Pointer` _returnvalue))
  (`UserWidget.AddToViewport` _output_get 500))

(event `/Game/Blueprints/Interfaces/BPI_InteractionSystem.DestroyPointer`
  (`/Engine/EditorBlueprintResources/StandardMacros.IsValid` (`self.GUI_Pointer`)
    (:`Is Valid`
      (`Widget.RemoveFromParent` (`self.GUI_Pointer`))
      (set `self.GUI_Pointer` null))))

(event `/Game/Blueprints/Interfaces/BPI_WeatherSystem.CreateTimeWidget`
  (params (WeatherSystem :type "/Game/Blueprints/Common/WeatherSystem/BP_WeatherSystem Object Reference"))
  (bind _returnvalue (`|CreateWidget` "/Game/GUI/HUD/HUD_Time.HUD_Time_C" null WeatherSystem))
  (bind _output_get (set `self.GUI_Time` _returnvalue))
  (`UserWidget.AddToViewport` _output_get 0))

(event `/Game/Blueprints/Interfaces/BPI_WeatherSystem.DestroyTimeWidget`
  (`/Engine/EditorBlueprintResources/StandardMacros.IsValid` (`self.GUI_Time`)
    (:`Is Valid`
      (`Widget.RemoveFromParent` (`self.GUI_Time`))
      (set `self.GUI_Time` null))))

(event `/Game/Blueprints/Interfaces/BPI_InteractionSystem.CreatePieMenu`
  (bind _returnvalue (`|CreateWidget` "/Game/GUI/HUD/HUD_PieMenu.HUD_PieMenu_C"))
  (set `self.GUI_PieMenu` _returnvalue))

(event `/Game/Blueprints/Interfaces/BPI_InteractionSystem.ShowPieMenu`
  (`/Engine/EditorBlueprintResources/StandardMacros.IsValid` (`self.GUI_PieMenu`)
    (:`Is Valid`
      (`UserWidget.AddToViewport` (`self.GUI_PieMenu`) 100)
      (`WidgetBlueprintLibrary.SetInputMode_GameAndUIEx` self (`self.GUI_PieMenu`)))))

(event `/Game/Blueprints/Interfaces/BPI_InteractionSystem.HidePieMenu`
  (`/Engine/EditorBlueprintResources/StandardMacros.IsValid` (`self.GUI_PieMenu`)
    (:`Is Valid`
      (`Widget.RemoveFromParent` (`self.GUI_PieMenu`))
      (`WidgetBlueprintLibrary.SetInputMode_GameOnly` self))))

(event `/Game/Blueprints/Interfaces/BPI_InteractionSystem.DestroyPieMenu`
  (`/Engine/EditorBlueprintResources/StandardMacros.IsValid` (`self.GUI_PieMenu`)
    (:`Is Valid`
      (`Widget.RemoveFromParent` (`self.GUI_PieMenu`))
      (set `self.GUI_PieMenu` null))))

(event `/Game/Blueprints/Interfaces/BPI_InteractionSystem.CreateConsumableWidget`
  (bind _returnvalue (`|CreateWidget` "/Game/GUI/HUD/HUD_Consumable.HUD_Consumable_C"))
  (bind _output_get (set `self.GUI_Consumable` _returnvalue))
  (`UserWidget.AddToViewport` _output_get 100))

(event `/Game/Blueprints/Interfaces/BPI_InteractionSystem.DestroyConsumableWidget`
  (`/Engine/EditorBlueprintResources/StandardMacros.IsValid` (`self.GUI_Consumable`)
    (:`Is Valid`
      (`Widget.RemoveFromParent` (`self.GUI_Consumable`))
      (set `self.GUI_Consumable` null))))

(event `/Game/Blueprints/Interfaces/BPI_InteractionSystem.UpdatePieMenu`
  (params (Consumable :type "/Game/Blueprints/Common/InteractionSystem/BP_ConsumableBase Object Reference"))
  (`/Engine/EditorBlueprintResources/StandardMacros.IsValid` (`self.GUI_PieMenu`)
    (:`Is Valid`
      (`/Game/GUI/HUD/HUD_PieMenu.UpdatePieMenuData` (`self.GUI_PieMenu`) Consumable))))

(event `/Game/Blueprints/Interfaces/BPI_InteractionSystem.UpdateConsumableWidget`
  (params (Consumable :type "/Game/Blueprints/Common/InteractionSystem/BP_ConsumableBase Object Reference"))
  (`/Engine/EditorBlueprintResources/StandardMacros.IsValid` (`self.GUI_Consumable`)
    (:`Is Valid`
      (`/Game/GUI/HUD/HUD_Consumable.UpdateConsumableData` (`self.GUI_Consumable`) Consumable))))

(event `/Game/Blueprints/Interfaces/BPI_InteractionSystem.AddDescriptionWidget`
  (params (POI :type "/Game/Blueprints/Common/POI/BP_POI Object Reference") (Interactable :type "/Game/Blueprints/Common/InteractionSystem/BP_InteractableBase Object Reference") (Text :type Text) (DelayBetweenLetters :type "Float (single-precision)"))
  (bind _returnvalue (`|CreateWidget` "/Game/GUI/HUD/HUD_Description.HUD_Description_C" null POI Interactable Text DelayBetweenLetters))
  (bind _output_get (set `self.GUI_Description` _returnvalue))
  (`UserWidget.AddToViewport` _output_get 2000))

(event `/Game/Blueprints/Interfaces/BPI_InteractionSystem.DestroyDescriptionWidget`
  (`/Engine/EditorBlueprintResources/StandardMacros.IsValid` (`self.GUI_Description`)
    (:`Is Valid`
      (`Widget.RemoveFromParent` (`self.GUI_Description`))
      (set `self.GUI_Description` null))))

(event `/Game/Blueprints/Interfaces/BPI_PlayerCharacter.CreateMapWidget`
  (params (RT_WorldMap :type "TextureRenderTarget2D Object Reference") (RT_Minimap :type "TextureRenderTarget2D Object Reference"))
  (bind _returnvalue (`|CreateWidget` "/Game/GUI/HUD/HUD_Map.HUD_Map_C" null RT_WorldMap RT_Minimap))
  (bind _output_get (set `self.GUI_Map` _returnvalue))
  (`UserWidget.AddToViewport` _output_get 1000))

(event `/Game/Blueprints/Interfaces/BPI_PlayerCharacter.DestroyMapWidget`
  (`/Engine/EditorBlueprintResources/StandardMacros.IsValid` (`self.GUI_Map`)
    (:`Is Valid`
      (`Widget.RemoveFromParent` (`self.GUI_Map`))
      (set `self.GUI_Map` null))))

(event `/Game/Blueprints/Interfaces/BPI_PlayerCharacter.UpdateMapWidget`
  (params (bMinimap :type Boolean))
  (`/Engine/EditorBlueprintResources/StandardMacros.IsValid` (`self.GUI_Map`)
    (:`Is Valid`
      (`/Game/GUI/HUD/HUD_Map.UpdateMapStatus` (`self.GUI_Map`) bMinimap)
      (if bMinimap
        (set `self.bShowMouseCursor` false)
        (set `self.bMinimap` true)
        (`WidgetBlueprintLibrary.SetInputMode_GameOnly` self)
        (else
          (set `self.bShowMouseCursor` true)
          (set `self.bMinimap` false)
          (`WidgetBlueprintLibrary.SetInputMode_GameAndUIEx` self null "DoNotLock" false))))))

(event `/Game/Blueprints/Interfaces/BPI_PlayerCharacter.CreateMapEdgeMarkerWidget`
  (params (MarkerData :type "/Game/Blueprints/Structures/FCommonMarker Structure") (Location :type "Vector Structure") (MinimapSizeInUnits :type "Float (single-precision)") (Owner :type "/Game/Blueprints/Common/Map/BP_CommonMarker Object Reference"))
  (`/Engine/EditorBlueprintResources/StandardMacros.IsValid` (`self.GUI_Map`)
    (:`Is Valid`
      (`/Game/GUI/HUD/HUD_Map.CreateMapEdgeMarker` (`self.GUI_Map`) MarkerData Location MinimapSizeInUnits Owner))))

(event `/Game/Blueprints/Interfaces/BPI_PlayerCharacter.DestroyMapEdgeMarkerWidget`
  (params (WidgetToDestroy :type "/Game/GUI/HUD/HUD_MapEdgeMarker Object Reference"))
  (`/Engine/EditorBlueprintResources/StandardMacros.IsValid` (`self.GUI_Map`)
    (:`Is Valid`
      (`/Game/GUI/HUD/HUD_Map.DestroyMapEdgeMarker` (`self.GUI_Map`) WidgetToDestroy))))

(event `/Game/Blueprints/Interfaces/BPI_InteractionSystem.CreateSaveWidget`
  (bind _returnvalue (`|CreateWidget` "/Game/GUI/HUD/HUD_SaveGame.HUD_SaveGame_C"))
  (bind _output_get (set `self.GUI_SaveGame` _returnvalue))
  (`UserWidget.AddToViewport` _output_get 100))

(event `/Game/Blueprints/Interfaces/BPI_QuestSystem.CreateQuestWidget`
  (bind _returnvalue (`|CreateWidget` "/Game/GUI/HUD/HUD_Quest.HUD_Quest_C"))
  (bind _output_get (set `self.GUI_Quest` _returnvalue))
  (`UserWidget.AddToViewport` _output_get 100))

(event `/Game/Blueprints/Interfaces/BPI_QuestSystem.DestroyQuestWidget`
  (`/Engine/EditorBlueprintResources/StandardMacros.IsValid` (`self.GUI_Quest`)
    (:`Is Valid`
      (`Widget.RemoveFromParent` (`self.GUI_Quest`))
      (set `self.GUI_Quest` null))))

(event `/Game/Blueprints/Interfaces/BPI_PlayerCharacter.CreateThreat`
  (params (Direction :type "Vector Structure") (Lifetime :type "Float (single-precision)"))
  (bind _returnvalue (`|CreateWidget` "/Game/GUI/HUD/HUD_IncomingThreat.HUD_IncomingThreat_C" null Direction Lifetime))
  (bind _output_get (set `self.GUI_IncomingThreat` _returnvalue))
  (`UserWidget.AddToViewport` _output_get 0)
  (`KismetArrayLibrary.Array_Add` (`self.GUI_IncomingThreatList`) (`self.GUI_IncomingThreat`))
  (if (and (`KismetArrayLibrary.Array_IsValidIndex` (`self.GUI_IncomingThreatList`)) (> (`KismetArrayLibrary.Array_Length` (`self.GUI_IncomingThreatList`)) 3))
    (`/Game/Blueprints/Interfaces/BPI_PlayerCharacter.RemoveThreat` (`|GetArrayItem` (`self.GUI_IncomingThreatList`)))))

(event `/Game/Blueprints/Interfaces/BPI_PlayerCharacter.RemoveThreat`
  (params (Widget :type "/Game/GUI/HUD/HUD_IncomingThreat Object Reference"))
  (`/Engine/EditorBlueprintResources/StandardMacros.IsValid` Widget
    (:`Is Valid`
      (`Widget.RemoveFromParent` Widget)
      (`KismetArrayLibrary.Array_RemoveItem` (`self.GUI_IncomingThreatList`) Widget))))

(event `/Game/Blueprints/Interfaces/BPI_PlayerCharacter.CreateBinoculars`
  ;[1 1 1] Binoculars
  (bind _returnvalue (`|CreateWidget` "/Game/GUI/HUD/HUD_Binoculars.HUD_Binoculars_C"))
  (set `self.GUI_Binoculars` _returnvalue))

(event `/Game/Blueprints/Interfaces/BPI_PlayerCharacter.DestroyBinoculars`
  ;[1 1 1] Binoculars
  (`/Engine/EditorBlueprintResources/StandardMacros.IsValid` (`self.GUI_Binoculars`)
    (:`Is Valid`
      (`Widget.RemoveFromParent` (`self.GUI_Binoculars`))
      (set `self.GUI_Binoculars` null))))

(event `/Game/Blueprints/Interfaces/BPI_PlayerCharacter.ShowBinoculars`
  ;[1 1 1] Binoculars
  (`/Engine/EditorBlueprintResources/StandardMacros.IsValid` (`self.GUI_Binoculars`)
    (:`Is Valid`
      (`UserWidget.AddToViewport` (`self.GUI_Binoculars`) 0))))

(event `/Game/Blueprints/Interfaces/BPI_PlayerCharacter.HideBinoculars`
  ;[1 1 1] Binoculars
  (`/Engine/EditorBlueprintResources/StandardMacros.IsValid` (`self.GUI_Binoculars`)
    (:`Is Valid`
      (`Widget.RemoveFromParent` (`self.GUI_Binoculars`)))))

(event `/Game/Blueprints/Interfaces/BPI_Inventory.CreateInventory`
  ;[1 1 1] Inventory
  (bind _returnvalue (`|CreateWidget` "/Game/GUI/HUD/HUD_Inventory.HUD_Inventory_C"))
  (set `self.GUI_Inventory` _returnvalue))

(event `/Game/Blueprints/Interfaces/BPI_Inventory.DestroyInventory`
  ;[1 1 1] Inventory
  (`/Engine/EditorBlueprintResources/StandardMacros.IsValid` (`self.GUI_Inventory`)
    (:`Is Valid`
      (`Widget.RemoveFromParent` (`self.GUI_Inventory`))
      (set `self.GUI_Inventory` null))))

(event `/Game/Blueprints/Interfaces/BPI_Inventory.ShowInventory`
  ;[1 1 1] Inventory
  (`/Engine/EditorBlueprintResources/StandardMacros.IsValid` (`self.GUI_Inventory`)
    (:`Is Valid`
      (`UserWidget.AddToViewport` (`self.GUI_Inventory`) 1500)
      (set `self.bShowMouseCursor` true)
      (`WidgetBlueprintLibrary.SetInputMode_GameAndUIEx` self null "DoNotLock" false))))

(event `/Game/Blueprints/Interfaces/BPI_Inventory.HideInventory`
  ;[1 1 1] Inventory
  (`/Engine/EditorBlueprintResources/StandardMacros.IsValid` (`self.GUI_Inventory`)
    (:`Is Valid`
      (`Widget.RemoveFromParent` (`self.GUI_Inventory`))
      (set `self.bShowMouseCursor` false)
      (`WidgetBlueprintLibrary.SetInputMode_GameOnly` self))))

(fn `GetActiveConsumableWidget`
  (returns (GUI_Consumable :type "/Game/GUI/HUD/HUD_Consumable Object Reference"))
  (return (`self.GUI_Consumable`)))

(fn `GetBinoculars`
  (returns (Object :type "/Game/GUI/HUD/HUD_Binoculars Object Reference"))
  (return (`self.GUI_Binoculars`)))

(fn `GetBinocularsMod`
  (returns (Value :type "Float (double-precision)"))
  (return 0.0))

(fn `GetHealth`
  (returns (Percent :type "Float (double-precision)") (PredictedPercent :type "Float (double-precision)") (CurrentHealth :type "Float (double-precision)") (MaxHealth :type "Float (double-precision)") (DeltaHealth :type "Float (double-precision)"))
  (return 0.0 0.0 0.0 0.0 0.0))

(fn `GetMinimapData`
  (returns (MinimapSizeInUnits :type "Float (double-precision)") (bMinimap :type Boolean) (MinimapReference :type "/Game/Blueprints/Common/Map/BP_Map Object Reference"))
  (return 0.0 false null))

(fn `GetPieMenuWidget`
  (returns (GUI_PieMenu :type "/Game/GUI/HUD/HUD_PieMenu Object Reference"))
  (return (`self.GUI_PieMenu`)))

(fn `GetPlayerData`
  (returns (PlayerData :type "/Game/Blueprints/Structures/GameDataChildren/FPlayerData Structure"))
  (return))

(fn `GetQuestWidget`
  (returns (GUI_Quest :type "/Game/GUI/HUD/HUD_Quest Object Reference"))
  (return (`self.GUI_Quest`)))

(fn `GetStamina`
  (returns (Stamina :type "Float (double-precision)") (Percent :type "Float (double-precision)") (bRunoutStamina :type Boolean))
  (return 0.0 0.0 false))

(fn `UserConstructionScript`)