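; BP_PlayerStart spawns and possesses the player character when a level begins, restoring state from saved game data.
; A transform saved for the current level takes priority; otherwise it spawns at its own transform, taking health and stamina from the save, or its defaults if NewScenario is set.
; On that first visit, a looping timer waits for the inventory to be ready, then saves.
; An Editor flag bypasses saved data.
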(event `self.ReceiveBeginPlay`
  (bind ((`Health_4_88425CE247140BDE2CFA078D066835A6` _health) (`Stamina_5_4D9EFE5640142286854514923DB7777D` _stamina)) (break `/Game/Blueprints/Structures/GameDataChildren/FPlayerData` (`.Player_34_DD80CB954E9A40AF1BD1338114B3921E` (break `/Game/Blueprints/Structures/FGameData` (`self.GameData`)))))
  (bind ((`Health_4_88425CE247140BDE2CFA078D066835A6` _health_2) (`Stamina_5_4D9EFE5640142286854514923DB7777D` _stamina_2)) (break `/Game/Blueprints/Structures/GameDataChildren/FPlayerData` (`.Player_34_DD80CB954E9A40AF1BD1338114B3921E` (break `/Game/Blueprints/Structures/FGameData` (`self.GameData`)))))
  (bind (_value _returnvalue) (`BlueprintMapLibrary.Map_Find` (`.LevelsPlayerTransform_37_88425CE247140BDE2CFA078D066835A6` (break `/Game/Blueprints/Structures/GameDataChildren/FLevelData` (`.Level_37_C2FF1CFD417204E825B165B1F75E41BE` (break `/Game/Blueprints/Structures/FGameData` (`self.GameData`))))) (`self.CurrentLevel`)))
  (if (not (`self.bEditor`))
    (bind _gamedata (message `/Game/Blueprints/Interfaces/BPI_GameInstance.LoadGameData` (`GameplayStatics.GetGameInstance`)))
    (set `self.GameData` _gamedata)
    (bind _returnvalue_2 (`GameplayStatics.GetCurrentLevelName` true))
    (set `self.CurrentLevel` _returnvalue_2)
    (if _returnvalue
      (set `self.SpawnTransform` _value)
      (bind _returnvalue_3 (`|SpawnActorFromClass` "/Game/Blueprints/Core/BP_PlayerCharacter.BP_PlayerCharacter_C" (`self.SpawnTransform`) "Undefined" "OverrideRootScale" null 300.0 _health_2 _stamina_2 (`self.QuestDB`) null))
      (set `self.PlayerCharacter` _returnvalue_3)
      (`Controller.Possess` (`GameplayStatics.GetPlayerController` 0) (`self.PlayerCharacter`))
      (else
        (set `self.SpawnTransform` (`self.GetTransform`))
        (if (`self.bNewScenario`)
          (bind _returnvalue_4 (`|SpawnActorFromClass` "/Game/Blueprints/Core/BP_PlayerCharacter.BP_PlayerCharacter_C" (`self.SpawnTransform`) "Undefined" "OverrideRootScale" null 300.0 (`self.Health`) (`self.Stamina`) (`self.QuestDB`) null))
          (set `self.PlayerCharacter` _returnvalue_4)
          (else
            (bind _returnvalue_5 (`|SpawnActorFromClass` "/Game/Blueprints/Core/BP_PlayerCharacter.BP_PlayerCharacter_C" (`self.SpawnTransform`) "Undefined" "OverrideRootScale" null 300.0 _health _stamina (`self.QuestDB`) null))
            (set `self.PlayerCharacter` _returnvalue_5)))
        (`Controller.Possess` (`GameplayStatics.GetPlayerController` 0) (`self.PlayerCharacter`))
        (bind _returnvalue_6 (`KismetSystemLibrary.K2_SetTimerDelegate` (`|CreateDelegate` :!event `CheckInventory`) 0.2 true))
        (set `self.CheckInventoryTimer` _returnvalue_6)))
    (else
      (bind _returnvalue_7 (`|SpawnActorFromClass` "/Game/Blueprints/Core/BP_PlayerCharacter.BP_PlayerCharacter_C" (`self.GetTransform`) "Undefined" "OverrideRootScale" null (`self.WalkSpeed`) (`self.Health`) (`self.Stamina`) (`self.QuestDB`) null))
      (set `self.PlayerCharacter` _returnvalue_7)
      (`Controller.Possess` (`GameplayStatics.GetPlayerController` 0) (`self.PlayerCharacter`)))))

(event `CheckInventory`
  (if (`/Game/Blueprints/Common/Inventory/BP_InventoryComponent.bInventoryReady` (`/Game/Blueprints/Core/BP_PlayerCharacter.InventoryComponent` (`self.PlayerCharacter`)))
    (`KismetSystemLibrary.K2_ClearAndInvalidateTimerHandle` (`self.CheckInventoryTimer`))
    (message `/Game/Blueprints/Interfaces/BPI_GameInstance.SaveGameData` (`GameplayStatics.GetGameInstance`))))

(fn `UserConstructionScript`)