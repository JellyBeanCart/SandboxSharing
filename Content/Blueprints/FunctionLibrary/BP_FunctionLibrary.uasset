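; Blueprint function library with shared lookups for the player character, map capture size and weather system, plus helpers that apply game settings.
; Getters cast player 0's character or fetch the first actor of the needed class in the level.
; ApplyGameSettings feeds brightness into the first PostProcessVolume's color gain by assigning a newly built settings struct.
; It also feeds sensitivity into player 0's controller input scales, with pitch negated.
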(fn `ApplyGameSettings`
  (params (Settings :type "/Game/Blueprints/Structures/FSettings Structure"))
  (`self.SetGlobalBrightness` (`.Brightness_2_B5A245054A4CF7FBDDF90B92A2A80A0F` (break `/Game/Blueprints/Structures/FSettings` (`local.Settings`))))
  (`self.SetGlobalSensitivity` (`.Sensitivity_4_BFD4E05F406D0FA57DD0ECBA4AF243EF` (break `/Game/Blueprints/Structures/FSettings` (`local.Settings`)))))

(fn `GetMapCaptureSize`
  (returns (MapSizeWorldUnits :type "Float (double-precision)") (MapSizeInKm :type "Float (double-precision)"))
  (bind _returnvalue (`GameplayStatics.GetActorOfClass` null "/Game/Blueprints/Common/Map/BP_MapCapture.BP_MapCapture_C"))
  (return (`/Game/Blueprints/Common/Map/BP_MapCapture.WorldSizeInUnits` _returnvalue) (`/Game/Blueprints/Common/Map/BP_MapCapture.WorldSizeInKm` _returnvalue)))

(fn `GetPlayerCharacter`
  (returns (PlayerCharacter :type "/Game/Blueprints/Core/BP_PlayerCharacter Object Reference"))
  (bind _asbp_player_character (cast `/Game/Blueprints/Core/BP_PlayerCharacter` (`GameplayStatics.GetPlayerCharacter` null)))
  (return _asbp_player_character))

(fn `GetWeatherSystem`
  (returns (Weather :type "/Game/Blueprints/Common/WeatherSystem/BP_WeatherSystem Object Reference"))
  (bind _returnvalue (`GameplayStatics.GetActorOfClass` null "/Game/Blueprints/Common/WeatherSystem/BP_WeatherSystem.BP_WeatherSystem_C"))
  (return _returnvalue))

(fn `SetGlobalBrightness`
  (params (Value :type "Float (double-precision)"))
  (bind _value (`local.Value`))
  (bind _returnvalue (`GameplayStatics.GetActorOfClass` null "/Script/Engine.PostProcessVolume"))
  (`/Engine/EditorBlueprintResources/StandardMacros.IsValid` _returnvalue
    (:`Is Valid`
      (set `PostProcessVolume.Settings` (make `PostProcessSettings` :`ColorGain` (`KismetMathLibrary.MakeVector4` _value _value _value _value)) _returnvalue))))

(fn `SetGlobalSensitivity`
  (params (Value :type "Float (double-precision)"))
  (set `PlayerController.InputYawScale` (`local.Value`) (`GameplayStatics.GetPlayerController` null))
  (set `PlayerController.InputPitchScale` (* (`local.Value`) -1.0) (`GameplayStatics.GetPlayerController` null))
  (set `PlayerController.InputRollScale` (`local.Value`) (`GameplayStatics.GetPlayerController` null)))